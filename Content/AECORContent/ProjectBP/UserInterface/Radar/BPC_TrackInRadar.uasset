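; Actor component that registers its owner on the player's radar in FlyingGameHUD when play begins.
; A RadarCategory switch routes the owner to the HUD's flying enemy, ground enemy, boss or pickup add function.
; Category names differ from those radar groups, and Vehicle shares the ground enemy branch with Special Creature.
; EventRemoveFromRadar mirrors the routing for removal, but nothing connected in this component calls it.
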(event Custom|EventAddToRadar
  (switch Utilities|FlowControl|Switch|SwitchonE_SonarCategories (Variables|Setup|GetRadarCategory)
    (:NewEnumerator1
      ;[1 1 1] Add Flying Enemy
      (bind _asflying_game_hud (Utilities|Casting|CastToFlyingGameHUD (HUD|GetHUD (Game|GetPlayerController 0))))
      (Default|FnAddtoRadarFlyingEnemy _asflying_game_hud (Components|GetOwner)))
    (:NewEnumerator2
      ;[1 1 1] Add Ground Enemy
      (bind _asflying_game_hud_2 (Utilities|Casting|CastToFlyingGameHUD (HUD|GetHUD (Game|GetPlayerController 0)) :!label _label))
      (Default|FnAddtoRadarGroundEnemy _asflying_game_hud_2 (Components|GetOwner)))
    (:NewEnumerator3
      ;[1 1 1] Add Boss
      (bind _asflying_game_hud_3 (Utilities|Casting|CastToFlyingGameHUD (HUD|GetHUD (Game|GetPlayerController 0))))
      (Default|FnAddtoRadarBosses _asflying_game_hud_3 (Components|GetOwner)))
    (:NewEnumerator5
      ;[1 1 1] Add PickUp
      (bind _asflying_game_hud_4 (Utilities|Casting|CastToFlyingGameHUD (HUD|GetHUD (Game|GetPlayerController 0))))
      (Default|FnAddtoRadarPickUp _asflying_game_hud_4 (Components|GetOwner)))
    (:NewEnumerator6
      (goto _label))))

(event Custom|EventRemoveFromRadar
  (switch Utilities|FlowControl|Switch|SwitchonE_SonarCategories (Variables|Setup|GetRadarCategory)
    (:NewEnumerator1
      ;[1 1 1] Remove Flying Enemy
      (bind _asflying_game_hud (Utilities|Casting|CastToFlyingGameHUD (HUD|GetHUD (Game|GetPlayerController 0))))
      (Default|FnRemovefromRadarFlyingEnemy _asflying_game_hud (Components|GetOwner)))
    (:NewEnumerator2
      ;[1 1 1] Remove Ground Enemy
      (bind _asflying_game_hud_2 (Utilities|Casting|CastToFlyingGameHUD (HUD|GetHUD (Game|GetPlayerController 0)) :!label _label))
      (Default|FnRemovefromRadarGroundEnemy _asflying_game_hud_2 (Components|GetOwner)))
    (:NewEnumerator3
      ;[1 1 1] Remove Boss
      (bind _asflying_game_hud_3 (Utilities|Casting|CastToFlyingGameHUD (HUD|GetHUD (Game|GetPlayerController 0))))
      (Default|FnRemovefromRadarBosses _asflying_game_hud_3 (Components|GetOwner)))
    (:NewEnumerator5
      ;[1 1 1] Remove PickUp
      (bind _asflying_game_hud_4 (Utilities|Casting|CastToFlyingGameHUD (HUD|GetHUD (Game|GetPlayerController 0))))
      (Default|FnRemovefromRadarPickUp _asflying_game_hud_4 (Components|GetOwner)))
    (:NewEnumerator6
      (goto _label))))

(event EventBeginPlay
  (CallFunction|EventAddtoRadar))