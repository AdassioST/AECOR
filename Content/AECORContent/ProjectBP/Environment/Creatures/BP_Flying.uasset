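; BP_Flying is a flying creature pawn that steers along a 3D navigation path.
; Each tick, once PathFound is set, it reads the Nav3D path and applies scaled movement input toward the current point.
; Coming within AcceptRadius advances PathIndex, capped at three below the path length, so it never targets the final two points.
; The path request and the setting of PathFound do not appear in these graphs.
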(event Collision|EventActorBeginOverlap
  (params (OtherActor :type Actor%20Object%20Reference)))

(event EventTick
  (params (DeltaSeconds :type Float%20%28single-precision%29))
  (bind _returnvalue (Transformation|GetActorLocation))
  (bind _self self)
  (bind _nav3d (Variables|BP_Flying_C|GetNav3D _self))
  (bind _path (Class|Nav3DComponent|GetPath _nav3d))
  (if (Variables|Default|GetPathFound)
    (if (<= (Math|Vector|Distance(Vector) _returnvalue (Utilities|Array|Get(acopy) _path (Variables|Default|GetPathIndex))) (Variables|Default|GetAcceptRadius))
      (bind _result (Math|Integer|IncrementInt (Variables|Default|GetPathIndex))
        (:%20%20
          (Variables|Default|SetPathIndex (Math|Integer|Min(Integer) _result (- (Utilities|Array|Length _path) 3))))))
    (Pawn|Input|AddMovementInput (Math|Vector|Normalize (- (Utilities|Array|Get(acopy) _path (Variables|Default|GetPathIndex)) _returnvalue)) 0.4 false))
  (|CallParentFunction DeltaSeconds))

(event EventBeginPlay
  (|CallParentFunction) ; This node is disabled and will not be called.\nDrag off pins to build functionality.
)

(fn ConstructionScript
  (|CallParentFunction))