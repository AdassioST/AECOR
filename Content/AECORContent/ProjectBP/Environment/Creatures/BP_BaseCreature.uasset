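; BP_BaseCreature is a base creature actor that provides health and death handling for creatures in the environment.
; Increase and decrease functions clamp health between zero and MaxCreatureHealth, with a drop below one calling CreatureDeath.
; Death prints the creature's name from its stats struct and destroys the actor.
; CorrectMovementDirection sets a yaw-only rotation derived from the actor's world location vector, rather than its velocity.
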(event Custom|CorrectMovementDirection
  (Transformation|SetActorRotation (Math|Rotator|MakeRotator 0.0 0.0 (.Yaw (Math|Rotator|BreakRotator (Math|Conversions|RotationFromXVector (Transformation|GetActorLocation)))))))

(event EventTick
  (params (DeltaSeconds :type Float%20%28single-precision%29)))

(fn ConstructionScript)

(fn IncreaseCreatureHealthValue
  (params (IncreaseAmount :type Float%20%28single-precision%29))
  (Variables|Default|SetCreatureHealth (Math|Float|Clamp(Float) (+ IncreaseAmount (Variables|Default|GetCreatureHealth)) 0.0 (Variables|Default|GetMaxCreatureHealth))))

(fn DecreaseCreatureHealthValue
  (params (DecreaseAmount :type Float%20%28single-precision%29))
  (Variables|Default|SetCreatureHealth (Math|Float|Clamp(Float) (- (Variables|Default|GetCreatureHealth) DecreaseAmount) 0.0 (Variables|Default|GetMaxCreatureHealth)))
  (if (< (Variables|Default|GetCreatureHealth) 1.0)
    (CallFunction|CreatureDeath)
    (return)
    (else
      (return))))

(fn CreatureDeath
  (Development|PrintString (Utilities|String|Append "The creature " (Utilities|String|ToString(Text) (.creaturename (Variables|CreatureStats|GetF_CreatureStats))) " has now died.") true true "(R=0.802994,G=1.000000,B=0.000000,A=1.000000)" 3.0)
  (Actor|DestroyActor))