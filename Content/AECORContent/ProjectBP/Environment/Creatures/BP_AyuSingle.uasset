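; Single Ayu fish creature actor that varies its colour by randomizing the materials on its static mesh.
; The construction script picks one of three sets at random (default, Gold or Vio) and assigns materials per slot for fins, body, eyes and tail.
; The Vio branch applies only the bottom fin material, as its other four assignments are disconnected and never run.
; The event graph has no active logic.
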(event EventBeginPlay
  (|CallParentFunction) ; This node is disabled and will not be called.\nDrag off pins to build functionality.
)

(event Collision|EventActorBeginOverlap
  (params (OtherActor :type Actor%20Object%20Reference)))

(event EventTick
  (params (DeltaSeconds :type Float%20%28single-precision%29))
  (|CallParentFunction DeltaSeconds) ; This node is disabled and will not be called.\nDrag off pins to build functionality.
)

(fn ConstructionScript
  (bind _staticmesh (Variables|Default|GetStaticMesh))
  (|CallParentFunction)
  (switch int (Math|Random|RandomIntegerinRange 0 2)
    (:0
      (Rendering|Material|SetMaterial _staticmesh 0 "/Game/AECORContent/Visuals/Environments/Creatures/Ayu/Materials/M_AyuBottomFin.M_AyuBottomFin")
      (Rendering|Material|SetMaterial _staticmesh 1 "/Game/AECORContent/Visuals/Environments/Creatures/Ayu/Materials/M_AyuBody.M_AyuBody")
      (Rendering|Material|SetMaterial _staticmesh 2 "/Game/AECORContent/Visuals/Environments/Creatures/Ayu/Materials/M_AyuEyes.M_AyuEyes")
      (Rendering|Material|SetMaterial _staticmesh 3 "/Game/AECORContent/Visuals/Environments/Creatures/Ayu/Materials/M_AyuFins.M_AyuFins")
      (Rendering|Material|SetMaterial _staticmesh 4 "/Game/AECORContent/Visuals/Environments/Creatures/Ayu/Materials/M_AyuTail.M_AyuTail"))
    (:1
      (Rendering|Material|SetMaterial _staticmesh 0 "/Game/AECORContent/Visuals/Environments/Creatures/Ayu/Materials/M_AyuBottomFinGold.M_AyuBottomFinGold")
      (Rendering|Material|SetMaterial _staticmesh 1 "/Game/AECORContent/Visuals/Environments/Creatures/Ayu/Materials/M_AyuBodyGold.M_AyuBodyGold")
      (Rendering|Material|SetMaterial _staticmesh 2 "/Game/AECORContent/Visuals/Environments/Creatures/Ayu/Materials/M_AyuEyesGold.M_AyuEyesGold")
      (Rendering|Material|SetMaterial _staticmesh 3 "/Game/AECORContent/Visuals/Environments/Creatures/Ayu/Materials/M_AyuFinsGold.M_AyuFinsGold")
      (Rendering|Material|SetMaterial _staticmesh 4 "/Game/AECORContent/Visuals/Environments/Creatures/Ayu/Materials/M_AyuTailGold.M_AyuTailGold"))
    (:2
      (Rendering|Material|SetMaterial _staticmesh 0 "/Game/AECORContent/Visuals/Environments/Creatures/Ayu/Materials/M_AyuBottomFinVio.M_AyuBottomFinVio"))))