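; Base location trigger that reveals a named world location the first time the player reaches it.
; Overlap on the LocationRange component accepts an actor whose display name is AE_MyCharacter, or a BP_BaseVehicle whose VehicleInfo class equals BP_BaseVehicle.
; Discovery shows the UI_WorldDiscovery widget with the location name, awards knowledge points to the cached player character and plays a melody.
; An AlreadyFound flag blocks repeat discoveries.
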(event OnComponentBeginOverlap(LocationRange)
  (params (OverlappedComponent :type Primitive%20Component%20Object%20Reference) (OtherActor :type Actor%20Object%20Reference) (OtherComp :type Primitive%20Component%20Object%20Reference) (OtherBodyIndex :type Integer) (bFromSweep :type Boolean) (SweepResult :type Hit%20Result%20Structure%20%28by%20ref%29))
  (if (Utilities|Enum|Equal(Enum) (Utilities|GetDisplayName OtherActor) "AE_MyCharacter")
    (CallFunction|ShowNewLocationDiscovered)
    (else
      (bind _asbp_base_vehicle (Utilities|Casting|CastToBP_BaseVehicle OtherActor))
      (if (== (Utilities|Struct|BreakF_VehicleInfo (Variables|/Game/AECORContent/ProjectBP/Environment/Interactables/Vehicles/BP_BaseVehicle.BP_BaseVehicle_C|GetVehicleInfo _asbp_base_vehicle)) "/Game/AECORContent/ProjectBP/Environment/Interactables/Vehicles/BP_BaseVehicle.BP_BaseVehicle_C")
        (CallFunction|ShowNewLocationDiscovered)))))

(event EventBeginPlay
  (bind _asae_my_character (Utilities|Casting|CastToAE_MyCharacter (Game|GetPlayerCharacter 0)))
  (Variables|Default|SetCharacterReference _asae_my_character))

(fn ConstructionScript)

(fn ShowNewLocationDiscovered
  (if (not (Variables|Default|GetAlreadyFound))
    (bind _returnvalue (UserInterface|CreateWidget "/Game/AECORContent/ProjectBP/UserInterface/PopUps/UI_WorldDiscovery.UI_WorldDiscovery_C"))
    (UserInterface|Viewport|AddtoViewport _returnvalue 0)
    (Default|IncreaseWorldKnowledgePoints (Variables|Default|GetCharacterReference) (Variables|Default|GetLocationKnowledgePoints))
    (Audio|PlaySound2D (Variables|Default|GetLocationDiscoveryMelody) 1.0 1.0 0.0 0 0)
    (Default|UpdateLocationName _returnvalue (Variables|Default|GetLocationName))
    (Variables|Default|SetAlreadyFound true)))