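; Base Blueprint for development modules that act as crafting stations for the player.
; When the player character enters the RangeArea, it sets the character's CraftingStation to the type stored in ModuleInfo.
; Leaving the area resets that value to the enum's first entry, without checking for other overlapping modules.
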(event OnComponentBeginOverlap(RangeArea)
  (params (OverlappedComponent :type Primitive%20Component%20Object%20Reference) (OtherActor :type Actor%20Object%20Reference) (OtherComp :type Primitive%20Component%20Object%20Reference) (OtherBodyIndex :type Integer) (bFromSweep :type Boolean) (SweepResult :type Hit%20Result%20Structure%20%28by%20ref%29))
  (bind _returnvalue (Game|GetPlayerCharacter 0))
  (if (== OtherActor _returnvalue)
    (bind _asae_my_character (Utilities|Casting|CastToAE_MyCharacter _returnvalue))
    (Variables|/Game/AECORContent/ProjectBP/MainConfiguration/AE_MyCharacter.AE_MyCharacter_C|SetCraftingStation _asae_my_character (Utilities|Struct|BreakF_ModuleInfo (Variables|Default|GetModuleInfo)))))

(event OnComponentEndOverlap(RangeArea)
  (params (OverlappedComponent :type Primitive%20Component%20Object%20Reference) (OtherActor :type Actor%20Object%20Reference) (OtherComp :type Primitive%20Component%20Object%20Reference) (OtherBodyIndex :type Integer))
  (bind _returnvalue (Game|GetPlayerCharacter 0))
  (if (== OtherActor _returnvalue)
    (bind _asae_my_character (Utilities|Casting|CastToAE_MyCharacter _returnvalue))
    (Variables|/Game/AECORContent/ProjectBP/MainConfiguration/AE_MyCharacter.AE_MyCharacter_C|SetCraftingStation _asae_my_character "NewEnumerator0")))

(event EventBeginPlay
  (|CallParentFunction) ; This node is disabled and will not be called.\nDrag off pins to build functionality.
)

(event Collision|EventActorBeginOverlap
  (params (OtherActor :type Actor%20Object%20Reference)))

(fn ConstructionScript
  (|CallParentFunction))