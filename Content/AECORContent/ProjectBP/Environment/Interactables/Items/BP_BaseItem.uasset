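; BP_BaseItem is the base Blueprint for interactable item pickups in the world.
; On Interaction, it checks that the instigator has inventory space, sends it the ItemInfo struct through PickUpMessage, then destroys itself.
; The construction script rebuilds ItemInfo with the actor's own class filled in, so the data passed on pickup records which item class it came from.
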(event EventInteraction
  (params (Instigator :type AE%20My%20Character%20Object%20Reference))
  (if (Default|HasSpaceinInventory Instigator)
    (Class|BPIInteract|PickUp(Message) Instigator (Variables|Default|GetItemInfo))
    (Actor|DestroyActor)))

(fn ConstructionScript
  (|CallParentFunction)
  (Variables|Default|SetItemInfo (Utilities|Struct|MakeF_ItemInfo (.itemtype (Variables|Default|GetItemInfo)) (.itemname (Variables|Default|GetItemInfo)) (.itemimage (Variables|Default|GetItemInfo)) (.itemid (Variables|Default|GetItemInfo)) (.itemrarity (Variables|Default|GetItemInfo)) (.itemdensity (Variables|Default|GetItemInfo)) (.itemindex (Variables|Default|GetItemInfo)) (Utilities|GetClass self) (.itemslot (Variables|Default|GetItemInfo)) (.itemvalue (Variables|Default|GetItemInfo)))))