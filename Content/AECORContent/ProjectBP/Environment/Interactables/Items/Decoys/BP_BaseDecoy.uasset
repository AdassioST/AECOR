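; BP_BaseDecoy is the base Blueprint for decoy items, which open a decoy creation UI when used from an item slot.
; UseSlotItem calls its parent, toggles the player character's inventory, then creates UI_DecoyCreation with the decoy and item info.
; It adds that widget to the viewport, focuses it in Game and UI input mode and shows the cursor.
; The PassDecoyReference event stores the ItemInfo handed to that widget.
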(event EventBeginPlay)

(event Collision|EventActorBeginOverlap
  (params (OtherActor :type Actor%20Object%20Reference)))

(event EventPassDecoyReference
  (params (ItemInfo :type F%20Item%20Info%20Structure))
  (Variables|Default|SetItemInfo ItemInfo))

(event EventTick
  (params (DeltaSeconds :type Float%20%28single-precision%29)))

(fn ConstructionScript
  (|CallParentFunction))

(fn UseSlotItem
  (bind _returnvalue (Game|GetPlayerController 0))
  (|CallParentFunction)
  (bind _asae_my_character (Utilities|Casting|CastToAE_MyCharacter (Game|GetPlayerCharacter 0)))
  (Default|ToggleInventory _asae_my_character)
  (bind _returnvalue_2 (UserInterface|CreateWidget "/Game/AECORContent/ProjectBP/UserInterface/Decoys/UI_DecoyCreation.UI_DecoyCreation_C"))
  (Variables|/Game/AECORContent/ProjectBP/UserInterface/Decoys/UI_DecoyCreation.UI_DecoyCreation_C|SetDecoyInfo _returnvalue_2 (Variables|Default|GetDecoyInfo))
  (Variables|/Game/AECORContent/ProjectBP/UserInterface/Decoys/UI_DecoyCreation.UI_DecoyCreation_C|SetItemInfo _returnvalue_2 (Variables|Default|GetItemInfo))
  (UserInterface|Viewport|AddtoViewport _returnvalue_2 3)
  (Input|SetInputModeGameandUI _returnvalue _returnvalue_2 "DoNotLock" true)
  (Variables|/Script/Engine.PlayerController|SetbShowMouseCursor _returnvalue true)
  (return true))