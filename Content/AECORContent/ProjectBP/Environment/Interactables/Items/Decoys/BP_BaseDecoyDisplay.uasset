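; BP_BaseDecoyDisplay is a display actor that shows a decoy's icon and colored landmark name.
; PassDecoyInfo creates a canvas render target, whose update callback draws the name and feeds it into a dynamic material on the DecoyText component.
; RefreshDecoyDisplay separately maps the icon enum to a minimap texture on the DecoyIcon component's dynamic material.
; Debug prints remain, and the camera-facing rotation logic is disconnected.
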(event Custom|DrawTextTexture
  (params (Canvas :type Canvas%20Object%20Reference) (Width :type Integer) (Height :type Integer))
  (bind _decoytext (Variables|Default|GetDecoyText))
  (Canvas|DrawTexture :self Canvas :RenderTexture "/Game/InfinityBladeGrassLands/Effects/FX_Textures/Tile/T_Black_32.T_Black_32" :ScreenSize (Math|Vector2D|MakeVector2D (Math|Conversions|ToFloat(Integer) Width) (Math|Conversions|ToFloat(Integer) Height)))
  (HUD|DrawText Canvas "/Game/AECORContent/ProjectBP/UserInterface/MainMenu/Font/AE_GameFont.AE_GameFont" (Utilities|String|ToString(Name) (.LandmarkName (Utilities|Struct|BreakF_DecoyInfo (stale EventPassDecoyInfo DecoyInfo)))) "(X=15.000000,Y=15.000000)" "(X=60.000000,Y=60.000000)" (.DecoyColor (Utilities|Struct|BreakF_DecoyInfo (stale EventPassDecoyInfo DecoyInfo))) 0.0 "(R=0.000000,G=0.000000,B=0.000000,A=1.000000)" "(X=1.000,Y=1.000)" false false false "(R=0.000000,G=0.936326,B=1.000000,A=1.000000)")
  (bind _returnvalue (Rendering|Material|CreateDynamicMaterialInstance _decoytext 0 "/Game/AECORContent/ProjectBP/Environment/Interactables/Items/Decoys/M_DecoyText_Inst.M_DecoyText_Inst" "None" :!class /Script/Engine.PrimitiveComponent))
  (Rendering|Material|SetMaterial _decoytext 0 _returnvalue)
  (Rendering|Material|SetTextureParameterValue _returnvalue "DecoyText" (Variables|Default|GetTextTexture))
  (Development|PrintString "Hello" true true "(R=1.000000,G=0.359989,B=0.000000,A=1.000000)"))

(event EventBeginPlay)

(event Collision|EventActorBeginOverlap
  (params (OtherActor :type Actor%20Object%20Reference)))

(event EventTick
  (params (DeltaSeconds :type Float%20%28single-precision%29)))

(event EventPassDecoyInfo
  (params (DecoyInfo :type F%20Decoy%20Info%20Structure))
  (Development|PrintString "Hello" true true "(R=0.000000,G=1.000000,B=0.088038,A=1.000000)")
  (bind _returnvalue (CanvasRenderTarget2D|CreateCanvasRenderTarget2D "/Script/Engine.CanvasRenderTarget2D" 1024 1024))
  (bind _output_get (Variables|Default|SetTextTexture _returnvalue))
  (EventDispatchers|BindEventtoOnCanvasRenderTargetUpdate _output_get (delegate Custom|DrawTextTexture))
  (Class|CanvasRenderTarget2D|UpdateResource _output_get))

(fn ConstructionScript)

(fn RefreshDecoyDisplay
  (params (InputDecoyInfo :type F%20Decoy%20Info%20Structure))
  (CallFunction|SelectDecoyIcon (Utilities|Struct|BreakF_DecoyInfo InputDecoyInfo))
  (return InputDecoyInfo))

(fn SelectDecoyIcon
  (params (DecoyIcon :type E_DecoyIcons%20Enum :default "NewEnumerator0"))
  (bind _returnvalue (Rendering|Material|CreateDynamicMaterialInstance (Variables|Default|GetDecoyIcon) 0 "/Game/AECORContent/ProjectBP/Environment/Interactables/Items/Decoys/M_DecoyDisplay_Inst.M_DecoyDisplay_Inst" "None" :!class /Script/Engine.PrimitiveComponent))
  (switch Utilities|FlowControl|Switch|SwitchonE_DecoyIcons DecoyIcon
    (:NewEnumerator1
      (Variables|Default|SetTexture "/Game/AECORContent/ProjectBP/UserInterface/Radar/UIAssets/Minimap_Boss_Color.Minimap_Boss_Color"))
    (:NewEnumerator2
      (Variables|Default|SetTexture "/Game/AECORContent/ProjectBP/UserInterface/Radar/UIAssets/Minimap_FlyingEnemy_Down.Minimap_FlyingEnemy_Down"))
    (:NewEnumerator3
      (Variables|Default|SetTexture "/Game/AECORContent/ProjectBP/UserInterface/Radar/UIAssets/Minimap_GroundEnemy_Color.Minimap_GroundEnemy_Color"))
    (:NewEnumerator4
      (Variables|Default|SetTexture "/Game/AECORContent/ProjectBP/UserInterface/Radar/UIAssets/Minimap_PickUp.Minimap_PickUp"))
    (:NewEnumerator5
      (Variables|Default|SetTexture "/Game/AECORContent/ProjectBP/UserInterface/Radar/UIAssets/Minimap_Player_Color.Minimap_Player_Color")))
  (Rendering|Material|SetTextureParameterValue _returnvalue "DecoyIcon" (Variables|Default|GetTexture)))