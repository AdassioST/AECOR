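; Base harvestable resource actor that a player drains until it yields an item.
; Harvest starts a self-recursive short-Delay loop that lowers remaining life and updates a progress widget until the character's StopHarvesting is set.
; On depletion, it compares each MaterialDropChance index with a random integer, stopping at a match.
; A match adds the item to the character's inventory, shows an obtain-item popup and destroys the actor; without one, the actor remains.
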(event Custom|DecreaseHarvestBar
  (if (not (Variables|/Game/AECORContent/ProjectBP/MainConfiguration/AE_MyCharacter.AE_MyCharacter_C|GetStopHarvesting (stale EventHarvest CharacterReference)))
    (Variables|Default|SetCharacterReference (stale EventHarvest CharacterReference))
    (Utilities|IsValid (Variables|Default|GetHarvestUIReference)
      (:Is%20Valid
        (CallFunction|CheckProgress (stale EventHarvest HarvestAmount)))
      (:Is%20Not%20Valid
        (bind _returnvalue (UserInterface|CreateWidget "/Game/AECORContent/ProjectBP/UserInterface/Harvesting/UI_Harvest.UI_Harvest_C"))
        (bind _output_get (Variables|Default|SetHarvestUIReference _returnvalue))
        (UserInterface|Viewport|AddtoViewport _output_get 0)
        (CallFunction|CheckProgress (stale EventHarvest HarvestAmount))))
    (Utilities|FlowControl|Delay 0.0001)
    (CallFunction|DecreaseHarvestBar)))

(event EventBeginPlay
  (|CallParentFunction) ; This node is disabled and will not be called.\nDrag off pins to build functionality.
)

(event Collision|EventActorBeginOverlap
  (params (OtherActor :type Actor%20Object%20Reference)))

(event EventTick
  (params (DeltaSeconds :type Float%20%28single-precision%29)))

(event EventHarvest
  (params (HarvestAmount :type Float%20%28single-precision%29) (CharacterReference :type AE%20My%20Character%20Object%20Reference))
  (CallFunction|DecreaseHarvestBar))

(event EventPlayerStoppedHarvesting
  (Widget|RemovefromParent (Variables|Default|GetHarvestUIReference))
  (Variables|Default|SetHarvestUIReference 0))

(fn ConstructionScript
  (|CallParentFunction))

(fn CheckProgress
  (params (HarvestAmount :type Float%20%28single-precision%29))
  (bind _output_get (Variables|Default|SetHarvestCurrentLife (- (Variables|Default|GetHarvestCurrentLife) HarvestAmount)))
  (if (<= _output_get 0.0)
    (CallFunction|ResourceDepleted)
    (else
      (Default|UpdateProgress (Variables|Default|GetHarvestUIReference) (Variables|Default|GetHarvestCurrentLife) (Variables|Default|GetHarvestMaxLife)))))

(fn ResourceDepleted
  (Widget|RemovefromParent (Variables|Default|GetHarvestUIReference))
  (bind (_array_element _array_index) (Utilities|Array|ForEachLoopwithBreak (Variables|Default|GetMaterialDropChance) :!label _label)
    (:LoopBody
      (if (== _array_index (Math|Random|RandomIntegerinRange 0 (- (Variables|Default|GetMaxMaterials) 1)))
        (LocalVariables|SetFoundObject true)
        (goto _label Break)))
    (:Completed
      (if (LocalVariables|GetFoundObject)
        (Default|AddtoInventory (Variables|Default|GetCharacterReference) (Variables|/Game/AECORContent/ProjectBP/Environment/Interactables/Items/BP_BaseItem.BP_BaseItem_C|GetItemInfo _array_element))
        (bind _returnvalue (UserInterface|CreateWidget "/Game/AECORContent/ProjectBP/UserInterface/Harvesting/UI_ObtainItem.UI_ObtainItem_C"))
        (bind _output_get (Variables|Default|SetObtainItemReference _returnvalue))
        (Default|UpdateItemIcon _output_get (Variables|/Game/AECORContent/ProjectBP/Environment/Interactables/Items/BP_BaseItem.BP_BaseItem_C|GetItemInfo _array_element))
        (Default|UpdateItemName _output_get (Variables|/Game/AECORContent/ProjectBP/Environment/Interactables/Items/BP_BaseItem.BP_BaseItem_C|GetItemInfo _array_element))
        (UserInterface|Viewport|AddtoViewport _output_get 0)
        (Actor|DestroyActor)))))