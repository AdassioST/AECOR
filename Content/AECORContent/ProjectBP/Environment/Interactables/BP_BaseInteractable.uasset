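; BP_BaseInteractable is a base interactable actor that announces itself to the player character and can be visually highlighted.
; Overlaps on its RangeArea register the interactable with the overlapping AE_MyCharacter on entry and unregister it on exit.
; SetHighlight toggles custom depth rendering on its StaticMesh and mirrors that state to player character 0's IsObjectHighlighted flag.
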(event OnComponentBeginOverlap(RangeArea)
  (params (OverlappedComponent :type Primitive%20Component%20Object%20Reference) (OtherActor :type Actor%20Object%20Reference) (OtherComp :type Primitive%20Component%20Object%20Reference) (OtherBodyIndex :type Integer) (bFromSweep :type Boolean) (SweepResult :type Hit%20Result%20Structure%20%28by%20ref%29))
  (bind _asae_my_character (Utilities|Casting|CastToAE_MyCharacter OtherActor))
  (Class|BPIInteract|RegisterInteractable(Message) _asae_my_character self))

(event OnComponentEndOverlap(RangeArea)
  (params (OverlappedComponent :type Primitive%20Component%20Object%20Reference) (OtherActor :type Actor%20Object%20Reference) (OtherComp :type Primitive%20Component%20Object%20Reference) (OtherBodyIndex :type Integer))
  (bind _asae_my_character (Utilities|Casting|CastToAE_MyCharacter OtherActor))
  (Class|BPIInteract|UnregisterInteractable(Message) _asae_my_character self))

(fn ConstructionScript)

(fn SetHighlight
  (params (Highlight? :type Boolean))
  (bind _asae_my_character (Utilities|Casting|CastToAE_MyCharacter (Game|GetPlayerCharacter 0)))
  (Rendering|SetRenderCustomDepth (Variables|Default|GetStaticMesh) Highlight?)
  (Variables|/Game/AECORContent/ProjectBP/MainConfiguration/AE_MyCharacter.AE_MyCharacter_C|SetIsObjectHighlighted _asae_my_character Highlight?))