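; Base vehicle Blueprint that drives a physics-simulated static mesh with player throttle, pitch, yaw and optional roll, tuned by VehicleInfo.
; Axis inputs apply torque, while Tick damps spin, ramps or decays throttle and blends velocity toward the mesh's negative right vector.
; Non-player hits, gated by a four-second cooldown, play random crash sounds and subtract health based on world X velocity.
; Destruction at zero health only prints a warning.
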(event OnComponentHit(StaticMesh)
  (params (HitComponent :type Primitive%20Component%20Object%20Reference) (OtherActor :type Actor%20Object%20Reference) (OtherComp :type Primitive%20Component%20Object%20Reference) (NormalImpulse :type Vector :default "0, 0, 0") (Hit :type Hit%20Result%20Structure%20%28by%20ref%29))
  (bind _staticmesh (Variables|Default|GetStaticMesh))
  (if (not (== OtherActor (Game|GetPlayerCharacter 0)))
    (Utilities|FlowControl|DoOnce false :!label _label
      (:Completed
        (bind _returnvalue (Physics|GetPhysicsLinearVelocity _staticmesh "None"))
        (CallFunction|PlayRandomCollisionCrashSound (Transformation|GetWorldLocation _staticmesh))
        (bind _output_get (Variables|Default|SetVehicleHealth (Math|Float|Clamp(Float) (- (Variables|Default|GetVehicleHealth) (Math|Float|Absolute(Float) (/ (.X (Math|Vector|BreakVector _returnvalue)) 1e+02))) 0.0 (Variables|Default|GetMaxVehicleHealth))))
        (if (not (<= (Variables|Default|GetVehicleHealth) 0.0))
          (Development|PrintString (Utilities|String|ToString(Float) _output_get) true true "(R=0.962563,G=1.000000,B=0.000000,A=1.000000)")
          (else
            (CallFunction|DestroyVehicle)))
        (Utilities|FlowControl|Delay 4.0)
        (goto _label Reset)))))

(event Collision|EventActorBeginOverlap
  (params (OtherActor :type Actor%20Object%20Reference)))

(event EventTick
  (params (DeltaSeconds :type Float%20%28single-precision%29))
  (bind _staticmesh (Variables|Default|GetStaticMesh))
  ;[0.3134 1 0.1362] Correct Movement and Add Throttle
  (Utilities|FlowControl|Sequence
    (:then_0
      (CallFunction|ThrottleInput)
      (Class|PrimitiveComponent|AddTorqueinDegrees _staticmesh (/ (Math|Vector|NegateVector (Physics|GetPhysicsAngularVelocityinDegrees (Variables|Default|GetStaticMesh) "None")) 0.5) "None" true)
      (Physics|AddForce _staticmesh "0, 0, 0" "None" true)
      (CallFunction|CalculateVehicleSpeed))))

(event Input|ActionEvents|InputActionThrottleUp
  (params (Key :type Key%20Structure))
  (:Pressed
    (Variables|Default|SetThrottleUp true))
  (:Released
    (Variables|Default|SetThrottleUp false)))

(event Input|ActionEvents|InputActionThrottleDown
  (params (Key :type Key%20Structure))
  (:Pressed
    (Variables|Default|SetThrottleDown true))
  (:Released
    (Variables|Default|SetThrottleDown false)))

(event Input|AxisEvents|InputAxisMoveRight
  (params (AxisValue :type Float%20%28single-precision%29))
  ;[0 1 0.6115] Axis Movement
  (Class|PrimitiveComponent|AddTorqueinDegrees (Variables|Default|GetStaticMesh) (Math|Vector|Lerp(Vector) "0, 0, 0" (* (Math|Vector|GetUpVector (Variables|Default|GetStaticMesh)) (* AxisValue (.VehicleTractionControl (Utilities|Struct|BreakF_VehicleInfo (Variables|Default|GetVehicleInfo))))) 0.1) "None" true))

(event Input|AxisEvents|InputAxisMoveForward
  (params (AxisValue :type Float%20%28single-precision%29))
  ;[0 1 0.6115] Axis Movement
  (Class|PrimitiveComponent|AddTorqueinDegrees (Variables|Default|GetStaticMesh) (Math|Vector|Lerp(Vector) "0, 0, 0" (* (Math|Vector|GetForwardVector (Variables|Default|GetStaticMesh)) (* (* AxisValue -1.0) (.VehicleTractionControl (Utilities|Struct|BreakF_VehicleInfo (Variables|Default|GetVehicleInfo))))) 0.1) "None" true))

(event Input|AxisEvents|InputAxisVehicleRoll
  (params (AxisValue :type Float%20%28single-precision%29))
  (bind _vehicleinfo (Variables|Default|GetVehicleInfo))
  (bind (_vehicletractioncontrol _canvehicleroll) (Utilities|Struct|BreakF_VehicleInfo _vehicleinfo))
  ;[0 1 0.6115] Axis Movement
  (if _canvehicleroll
    (Class|PrimitiveComponent|AddTorqueinDegrees (Variables|Default|GetStaticMesh) (Math|Vector|Lerp(Vector) "0, 0, 0" (* (Math|Vector|GetRightVector (Variables|Default|GetStaticMesh)) (* AxisValue _vehicletractioncontrol)) 0.1) "None" true)))

(fn ConstructionScript)

(fn ThrottleInput
  (bind _vehicleinfo (Variables|Default|GetVehicleInfo))
  (bind _vehiclemaxthrottle (Utilities|Struct|BreakF_VehicleInfo _vehicleinfo))
  (bind _returnvalue (* _vehiclemaxthrottle -1.0))
  (if (Variables|Default|GetThrottleUp)
    (Variables|Default|SetVehicleThrottleAmount (Math|Float|Clamp(Float) (+ (Variables|Default|GetVehicleThrottleAmount) (Variables|Default|GetThrottleRecoveryRate)) _returnvalue _vehiclemaxthrottle))
    (elif (Variables|Default|GetThrottleDown)
      (Variables|Default|SetVehicleThrottleAmount (Math|Float|Clamp(Float) (- (Variables|Default|GetVehicleThrottleAmount) (Variables|Default|GetThrottleRecoveryRate)) _returnvalue _vehiclemaxthrottle))
      (else
        (CallFunction|RegulateThrottletoZero)))))

(fn CalculateVehicleSpeed
  (bind _vehicleinfo (Variables|Default|GetVehicleInfo))
  (bind _staticmesh (Variables|Default|GetStaticMesh))
  (bind _vehiclemaxspeed (Utilities|Struct|BreakF_VehicleInfo _vehicleinfo))
  (bind _returnvalue (Physics|GetPhysicsLinearVelocity _staticmesh "None"))
  (Physics|SetPhysicsLinearVelocity (Variables|Default|GetStaticMesh) (Math|Vector|Lerp(Vector) _returnvalue (* (Math|Vector|GetRightVector _staticmesh) (* (Math|Float|Clamp(Float) (* (Variables|Default|GetVehicleThrottleAmount) 2.5e+02) (* _vehiclemaxspeed -0.25) _vehiclemaxspeed) -1.0)) 0.01) false "None"))

(fn RegulateThrottletoZero
  (if (> (Variables|Default|GetVehicleThrottleAmount) 0.0)
    (Variables|Default|SetVehicleThrottleAmount (- (Variables|Default|GetVehicleThrottleAmount) (* (Variables|Default|GetThrottleRecoveryRate) 0.5)))
    (elif (< (Variables|Default|GetVehicleThrottleAmount) 0.0)
      (Variables|Default|SetVehicleThrottleAmount (+ (Variables|Default|GetVehicleThrottleAmount) (* (Variables|Default|GetThrottleRecoveryRate) 0.5))))))

(fn DestroyVehicle
  (Development|PrintString "Vehicle health is critical, it should be destroyed" true true "(R=1.000000,G=0.000000,B=0.028684,A=1.000000)"))

(fn PlayRandomCollisionCrashSound
  (params (SoundLocation :type Vector))
  (bind _vehicleinfo (Variables|Default|GetVehicleInfo))
  (bind _vehiclecrashplaylist (Utilities|Struct|BreakF_VehicleInfo _vehicleinfo))
  (bind _returnvalue (Utilities|Array|Length _vehiclecrashplaylist))
  (bind _returnvalue_2 (- _returnvalue 1))
  (bind _returnvalue_3 (Math|Random|RandomIntegerinRange 0 _returnvalue_2))
  (if (== (LocalVariables|GetLastSoundIndex) _returnvalue_3)
    (CallFunction|PlayRandomCollisionCrashSound SoundLocation)
    (else
      (Audio|PlaySoundatLocation (Utilities|Array|Get(acopy) _vehiclecrashplaylist _returnvalue_3) SoundLocation "0, 0, 0" 1.0 1.0 0.0 0 0 0)
      (LocalVariables|SetLastSoundIndex _returnvalue_3))))