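; BP_TempModifier is a placeable environment volume that changes the temperature affecting AE_MyCharacter actors inside it.
; On begin overlap it calls ApplyTemperatureModifier on the character with an optional world temperature override and an additive area modifier.
; On end overlap it calls the same function with the override off and both values negated.
; The construction script sizes the capsule volume from the Radius and Height variables.
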(event OnComponentBeginOverlap(Volume)
  (params (OverlappedComponent :type Primitive%20Component%20Object%20Reference) (OtherActor :type Actor%20Object%20Reference) (OtherComp :type Primitive%20Component%20Object%20Reference) (OtherBodyIndex :type Integer) (bFromSweep :type Boolean) (SweepResult :type Hit%20Result%20Structure%20%28by%20ref%29))
  (bind _asae_my_character (Utilities|Casting|CastToAE_MyCharacter OtherActor))
  (Default|ApplyTemperatureModifier _asae_my_character (Variables|Default|GetOverrideLocalWorldTemp?) (Variables|Default|GetOverridenWorldTemp) (Variables|Default|GetAreaTemperatureModifier)))

(event OnComponentEndOverlap(Volume)
  (params (OverlappedComponent :type Primitive%20Component%20Object%20Reference) (OtherActor :type Actor%20Object%20Reference) (OtherComp :type Primitive%20Component%20Object%20Reference) (OtherBodyIndex :type Integer))
  (bind _asae_my_character (Utilities|Casting|CastToAE_MyCharacter OtherActor))
  (Default|ApplyTemperatureModifier _asae_my_character false (* (Variables|Default|GetOverridenWorldTemp) -1.0) (* (Variables|Default|GetAreaTemperatureModifier) -1.0)))

(fn ConstructionScript
  (Components|Capsule|SetCapsuleSize (Variables|Default|GetVolume) (Variables|VolumeSize|GetRadius) (Variables|VolumeSize|GetHeight) true))