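; Day-night cycle actor for an underwater environment that drives time, lighting, ocean look and world temperature.
; Tick advances the hour, rotates the sun and writes clock, day count and night flag to the player character.
; Sun pitch selects day or night transitions: timelines blend sky and ocean parameter collections, while self-recalling delayed events step sun, skylight and caustics.
; A looping timer derives temperature from a fluctuation curve over the hour.
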(event Custom|SetNIghtLightning
  (bind _sun (Variables|DayConfiguration|GetSun))
  (bind _skylight (Variables|DayConfiguration|GetSkylight))
  (bind _lightcomponent (Variables|/Script/Engine.Light|GetLightComponent _sun))
  (bind _lightcomponent_2 (Variables|/Script/Engine.SkyLight|GetLightComponent _skylight))
  (bind _intensity (Variables|/Script/Engine.LightComponentBase|GetIntensity _lightcomponent))
  (bind _intensity_2 (Variables|/Script/Engine.LightComponentBase|GetIntensity _lightcomponent_2))
  (bind _returnvalue (- _intensity 0.05))
  (bind _returnvalue_2 (- _intensity_2 0.005))
  (bind _returnvalue_3 (Math|Float|Clamp(Float) _returnvalue 0.00025 15.842632))
  (bind _returnvalue_4 (Math|Float|Clamp(Float) _returnvalue_2 0.01 0.75))
  ;[0.006005 0 0.06771] Transition to Night Time
  (bind _outalpha (Timeline|ColorTransitionNight Play)
    (:Update
      (DayNightTransition|RefreshOceanColouratNightTime _outalpha))
    (:Finished
      (Rendering|Components|Light|SetIntensity _lightcomponent _returnvalue_3)
      (Rendering|Components|Light|SetIntensity _lightcomponent_2 _returnvalue_4)
      (DayNightTransition|RefreshCausticsatNightTime)
      (if (and (<= _returnvalue_4 0.01) (<= _returnvalue_3 0.0025))
        (Variables|Default|SetHasNightLightningFinished true)
        (else
          (Utilities|FlowControl|Delay 0.01)
          (CallFunction|SetNIghtLightning))))))

(event Custom|SetDayLight
  (bind _sun (Variables|DayConfiguration|GetSun))
  (bind _skylight (Variables|DayConfiguration|GetSkylight))
  (bind _lightcomponent (Variables|/Script/Engine.Light|GetLightComponent _sun))
  (bind _lightcomponent_2 (Variables|/Script/Engine.SkyLight|GetLightComponent _skylight))
  (bind _intensity (Variables|/Script/Engine.LightComponentBase|GetIntensity _lightcomponent))
  (bind _intensity_2 (Variables|/Script/Engine.LightComponentBase|GetIntensity _lightcomponent_2))
  (bind _returnvalue (+ _intensity_2 0.005))
  (bind _returnvalue_2 (+ _intensity 0.05))
  (bind _returnvalue_3 (Math|Float|Clamp(Float) _returnvalue 0.01 0.75))
  (bind _returnvalue_4 (Math|Float|Clamp(Float) _returnvalue_2 0.0025 15.842632))
  ;[1 0.8185 0] Transition to Day Time
  (bind _outalpha (Timeline|ColorTransitionDay Play)
    (:Update
      (DayNightTransition|RefreshOceanColouratDayTime _outalpha))
    (:Finished
      (Rendering|Components|Light|SetIntensity _lightcomponent _returnvalue_4)
      (Rendering|Components|Light|SetIntensity _lightcomponent_2 _returnvalue_3)
      (DayNightTransition|RefreshCausticsatDayTime)
      (if (and (>= _returnvalue_3 1.25) (>= _returnvalue_4 1e+01))
        (Variables|Default|SetHasDayLightningFinished true)
        (else
          (Utilities|FlowControl|Delay 0.01)
          (CallFunction|SetDayLight))))))

(event EventBeginPlay
  ;[0.1767 0.5927 0.4742] Event Start-Up
  (Utilities|FlowControl|Sequence
    (:then_0
      (bind _asae_my_character (Utilities|Casting|CastToAE_MyCharacter (Game|GetPlayerCharacter 0)))
      (bind _output_get (Variables|Default|SetCharacterReference _asae_my_character)))
    (:then_1
      (bind _output_get_2 (Variables|DayConfiguration|SetOneDay (* (Variables|DayConfiguration|GetDayLengthInMinutes) 6e+01)))
      (Variables|/Game/AECORContent/ProjectBP/MainConfiguration/AE_MyCharacter.AE_MyCharacter_C|SetOneHour _output_get (/ _output_get_2 24.0)))
    (:then_2
      (Utilities|FlowControl|Delay 0.0001)
      (CallFunction|SetHudReference))
    (:then_3
      (CallFunction|StartUpdatingTemperature))))

(event EventTick
  (params (DeltaSeconds :type Float%20%28single-precision%29))
  (bind _sun (Variables|DayConfiguration|GetSun))
  ;[0 0.5003 1] Refresh Hour to In-Game Time
  (bind _output_get (Variables|DayConfiguration|SetHour (+ (Variables|DayConfiguration|GetHour) (/ DeltaSeconds (Variables|/Game/AECORContent/ProjectBP/MainConfiguration/AE_MyCharacter.AE_MyCharacter_C|GetOneHour (Variables|Default|GetCharacterReference))))))
  (CallFunction|Clock _output_get)
  (Utilities|FlowControl|Sequence
    (:then_0
      (if (>= _output_get 24.0)
        (Variables|DayConfiguration|SetHour 0.0)
        (Variables|/Game/AECORContent/ProjectBP/MainConfiguration/AE_MyCharacter.AE_MyCharacter_C|SetPassedDays (Variables|Default|GetCharacterReference) (+ (Variables|/Game/AECORContent/ProjectBP/MainConfiguration/AE_MyCharacter.AE_MyCharacter_C|GetPassedDays (Variables|Default|GetCharacterReference)) 1))))
    (:then_1
      (bind _output_get_2 (Variables|DayConfiguration|SetSunAngle (+ (* (/ _output_get 6.0) 9e+01) 9e+01)))
      (Transformation|SetActorRotation _sun (Math|Rotator|MakeRotator 0.0 _output_get_2 0.0))
      (Default|UpdateSunDirection (Variables|DayConfiguration|GetSkyDome))
      (bind _output_get_3 (Variables|/Game/AECORContent/ProjectBP/MainConfiguration/AE_MyCharacter.AE_MyCharacter_C|SetNightTime (Variables|Default|GetCharacterReference) (Math|Float|InRange(Float) (.pitch (Transformation|GetActorRotation _sun)) 25.0 125.0)))
      (if _output_get_3
        (if (not (Variables|Default|GetHasNightLightningFinished))
          (CallFunction|SetNIghtLightning)
          (bind (_direction _moon _glow _postprocess _skysphereday _skyspherenight) (Timeline|DayToNight Play)
            (:Update
              (Rendering|Material|SetScalarParameterValue "/Game/AECORContent/Visuals/Environments/Sky/MPC_Sky.MPC_Sky" "OpacityDay" _skysphereday :!class /Script/Engine.KismetMaterialLibrary)
              (Rendering|Material|SetScalarParameterValue "/Game/AECORContent/Visuals/Environments/Sky/MPC_Sky.MPC_Sky" "OpacityNight" _skyspherenight :!class /Script/Engine.KismetMaterialLibrary))
            (:Finished
              (Variables|Default|SetHasNightLightningFinished false)
              (Variables|Default|SetHasDayLightningFinished false))))
        (elif (not (Variables|Default|GetHasDayLightningFinished))
          (CallFunction|SetDayLight)
          (Timeline|DayToNight Reverse))))))

(fn ConstructionScript
  (bind _returnvalue (Rendering|Material|CreateDynamicMaterialInstance "/Game/Z_OceanAssets/Ocean/Materials/M_Underwater_PP_Inst2.M_Underwater_PP_Inst2" "None" :!class /Script/Engine.KismetMaterialLibrary))
  (Variables|Default|SetOceanColor _returnvalue))

(fn Clock
  (params (Time :type Float%20%28single-precision%29))
  (bind _characterreference (Variables|Default|GetCharacterReference))
  (bind _output_get (Variables|DayConfiguration|SetTime (Math|Timespan|MakeTimespan 0 0 0 (Math|Float|Truncate (* Time 3.6e+03)))))
  (if (and (>= (.Minutes (Math|Timespan|BreakTimespan _output_get)) 0) (<= (.Minutes (Math|Timespan|BreakTimespan _output_get)) 9))
    (Variables|/Game/AECORContent/ProjectBP/MainConfiguration/AE_MyCharacter.AE_MyCharacter_C|SetClock _characterreference (Utilities|Text|ToText(String) (Utilities|String|Append (Utilities|String|ToString(Integer) (Math|Float|Truncate (Math|Float|MapRangeClamped (Math|Conversions|ToFloat(Integer) (.Hours (Math|Timespan|BreakTimespan _output_get))) 0.0 24.0 0.0 37.0))) " : " "0" (Utilities|String|ToString(Integer) (.Minutes (Math|Timespan|BreakTimespan _output_get))))))
    (else
      (Variables|/Game/AECORContent/ProjectBP/MainConfiguration/AE_MyCharacter.AE_MyCharacter_C|SetClock _characterreference (Utilities|Text|ToText(String) (Utilities|String|Append (Utilities|String|ToString(Integer) (Math|Float|Truncate (Math|Float|MapRangeClamped (Math|Conversions|ToFloat(Integer) (.Hours (Math|Timespan|BreakTimespan _output_get))) 0.0 24.0 0.0 37.0))) " : " (Utilities|String|ToString(Integer) (.Minutes (Math|Timespan|BreakTimespan _output_get)))))))))

(fn StartUpdatingTemperature
  (Utilities|Time|SetTimerbyFunctionName self "UpdateWorldTemperature" (/ 1.0 (Variables|Temperature|GetTemperatureUpdateRate)) true))

(fn UpdateWorldTemperature
  (Variables|Temperature|SetFinalWorldTemperature (+ (* (Math|Curves|GetFloatValue (Variables|Temperature|GetTempFluctuationCurve) (Math|Float|%(Float) (/ (Variables|DayConfiguration|GetHour) 24.0) 1.0)) (Variables|Temperature|GetWorldTemperatureVariation)) (Variables|Temperature|GetBaseWorldTemperature))))

(fn SetHudReference
  (Utilities|IsValid (Variables|Default|GetHUDReference)
    (:Is%20Not%20Valid
      (bind _asae_my_character (Utilities|Casting|CastToAE_MyCharacter (Game|GetPlayerCharacter 0)))
      (Variables|Default|SetHUDReference (Variables|/Game/AECORContent/ProjectBP/MainConfiguration/AE_MyCharacter.AE_MyCharacter_C|GetHUD%20Reference _asae_my_character)))))

(fn RefreshCausticsatNightTime
  (bind _caustics (Variables|DayConfiguration|GetCaustics))
  (bind _lightcomponent (Variables|/Script/Engine.Light|GetLightComponent _caustics))
  (Rendering|Components|Light|SetIntensity _lightcomponent (Math|Float|Clamp(Float) (- (Variables|/Script/Engine.LightComponentBase|GetIntensity _lightcomponent) 0.05) 4.25 1e+01))
  (bind _returnvalue (Rendering|Material|GetScalarParameterValue "/Game/AECORContent/ProjectBP/PostProcess/UnderwaterCaustics/MPC_Caustics.MPC_Caustics" "PannerSpeedX" :!class /Script/Engine.KismetMaterialLibrary))
  (Rendering|Material|SetScalarParameterValue "/Game/AECORContent/ProjectBP/PostProcess/UnderwaterCaustics/MPC_Caustics.MPC_Caustics" "PannerSpeedX" (Math|Float|Clamp(Float) (- _returnvalue 0.01) 0.025 0.045) :!class /Script/Engine.KismetMaterialLibrary)
  (Rendering|Material|SetScalarParameterValue "/Game/AECORContent/ProjectBP/PostProcess/UnderwaterCaustics/MPC_Caustics.MPC_Caustics" "PannerSpeedY" (Math|Float|Clamp(Float) (- _returnvalue 0.01) 0.025 0.045) :!class /Script/Engine.KismetMaterialLibrary)
  (return))

(fn RefreshCausticsatDayTime
  (bind _caustics (Variables|DayConfiguration|GetCaustics))
  (bind _lightcomponent (Variables|/Script/Engine.Light|GetLightComponent _caustics))
  (Rendering|Components|Light|SetIntensity _lightcomponent (Math|Float|Clamp(Float) (+ (Variables|/Script/Engine.LightComponentBase|GetIntensity _lightcomponent) 0.05) 4.25 1e+01))
  (bind _returnvalue (Rendering|Material|GetScalarParameterValue "/Game/AECORContent/ProjectBP/PostProcess/UnderwaterCaustics/MPC_Caustics.MPC_Caustics" "PannerSpeedX" :!class /Script/Engine.KismetMaterialLibrary))
  (Rendering|Material|SetScalarParameterValue "/Game/AECORContent/ProjectBP/PostProcess/UnderwaterCaustics/MPC_Caustics.MPC_Caustics" "PannerSpeedX" (Math|Float|Clamp(Float) (+ _returnvalue 1e-05) 0.025 0.045) :!class /Script/Engine.KismetMaterialLibrary)
  (Rendering|Material|SetScalarParameterValue "/Game/AECORContent/ProjectBP/PostProcess/UnderwaterCaustics/MPC_Caustics.MPC_Caustics" "PannerSpeedY" (Math|Float|Clamp(Float) (+ _returnvalue 1e-05) 0.025 0.045) :!class /Script/Engine.KismetMaterialLibrary)
  (return))

(fn RefreshOceanColouratDayTime
  (params (OutAlpha :type Float%20%28single-precision%29))
  (Rendering|Material|SetVectorParameterValue "/Game/AECORContent/ProjectBP/PostProcess/UnderwaterCaustics/MPC_OceanColor.MPC_OceanColor" "ExponentialFogColor" (Class|KismetMathLibrary|LinearColorLerpUsingHSV (Variables|OceanColorShallowsNight|GetExponentialFogColorShallowsNight) (Variables|OceanColorShallowsDay|GetExponentialFogColorShallowsDay) OutAlpha) :!class /Script/Engine.KismetMaterialLibrary)
  (Rendering|Material|SetVectorParameterValue "/Game/AECORContent/ProjectBP/PostProcess/UnderwaterCaustics/MPC_OceanColor.MPC_OceanColor" "SceneColorDeep" (Class|KismetMathLibrary|LinearColorLerpUsingHSV (Variables|OceanColorShallowsNight|GetSceneColorDeepShallowsNight) (Variables|OceanColorShallowsDay|GetSceneColorDeepShallowsDay) OutAlpha) :!class /Script/Engine.KismetMaterialLibrary)
  (Rendering|Material|SetVectorParameterValue "/Game/AECORContent/ProjectBP/PostProcess/UnderwaterCaustics/MPC_OceanColor.MPC_OceanColor" "SceneColorShallow" (Class|KismetMathLibrary|LinearColorLerpUsingHSV (Variables|OceanColorShallowsNight|GetSceneColorShallowShallowsNight) (Variables|OceanColorShallowsDay|GetSceneColorShallowShallowsDay) OutAlpha) :!class /Script/Engine.KismetMaterialLibrary)
  (Rendering|Material|SetVectorParameterValue "/Game/AECORContent/ProjectBP/PostProcess/UnderwaterCaustics/MPC_OceanColor.MPC_OceanColor" "SunColor" (Class|KismetMathLibrary|LinearColorLerpUsingHSV (Variables|OceanColorShallowsNight|GetSunColorShallowsNight) (Variables|OceanColorShallowsDay|GetSunColorShallowsDay) OutAlpha) :!class /Script/Engine.KismetMaterialLibrary))

(fn RefreshOceanColouratNightTime
  (params (OutAlpha :type Float%20%28single-precision%29))
  (Rendering|Material|SetVectorParameterValue "/Game/AECORContent/ProjectBP/PostProcess/UnderwaterCaustics/MPC_OceanColor.MPC_OceanColor" "ExponentialFogColor" (Class|KismetMathLibrary|LinearColorLerpUsingHSV (Variables|OceanColorShallowsNight|GetExponentialFogColorShallowsNight) (Variables|OceanColorShallowsDay|GetExponentialFogColorShallowsDay) OutAlpha) :!class /Script/Engine.KismetMaterialLibrary)
  (Rendering|Material|SetVectorParameterValue "/Game/AECORContent/ProjectBP/PostProcess/UnderwaterCaustics/MPC_OceanColor.MPC_OceanColor" "SceneColorDeep" (Class|KismetMathLibrary|LinearColorLerpUsingHSV (Variables|OceanColorShallowsNight|GetSceneColorDeepShallowsNight) (Variables|OceanColorShallowsDay|GetSceneColorDeepShallowsDay) OutAlpha) :!class /Script/Engine.KismetMaterialLibrary)
  (Rendering|Material|SetVectorParameterValue "/Game/AECORContent/ProjectBP/PostProcess/UnderwaterCaustics/MPC_OceanColor.MPC_OceanColor" "SceneColorShallow" (Class|KismetMathLibrary|LinearColorLerpUsingHSV (Variables|OceanColorShallowsNight|GetSceneColorShallowShallowsNight) (Variables|OceanColorShallowsDay|GetSceneColorShallowShallowsDay) OutAlpha) :!class /Script/Engine.KismetMaterialLibrary)
  (Rendering|Material|SetVectorParameterValue "/Game/AECORContent/ProjectBP/PostProcess/UnderwaterCaustics/MPC_OceanColor.MPC_OceanColor" "SunColor" (Class|KismetMathLibrary|LinearColorLerpUsingHSV (Variables|OceanColorShallowsNight|GetSunColorShallowsNight) (Variables|OceanColorShallowsDay|GetSunColorShallowsDay) OutAlpha) :!class /Script/Engine.KismetMaterialLibrary))