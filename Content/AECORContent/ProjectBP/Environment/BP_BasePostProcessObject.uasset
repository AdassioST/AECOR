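; Base post-process object that toggles custom depth rendering on its skeletal and static meshes to match the player's thermal vision state.
; On BeginPlay it caches the player's AE_MyCharacter, then runs a self-rescheduling update on a RenderUpdateRate delay.
; Thermal vision turns custom depth on, otherwise it turns off.
; With thermal off and an object highlighted, it only calls GetBestInteractable, and the loop stops rescheduling.
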(event Custom|UpdatePostProcessRender
  (if (Variables|/Game/AECORContent/ProjectBP/Main/AE_MyCharacter.AE_MyCharacter_C|GetIsThermalVisionOn (stale EventBeginPlay _asae_my_character))
    (bind _output_get (Variables|Default|SetRenderCustomDepth true))
    (Rendering|SetRenderCustomDepth (Variables|Default|GetSkeletalMesh) _output_get)
    (Rendering|SetRenderCustomDepth (Variables|Default|GetStaticMesh) _output_get)
    (Utilities|FlowControl|Delay (Variables|Default|GetRenderUpdateRate) :!label _label)
    (CallFunction|UpdatePostProcessRender)
    (elif (Variables|/Game/AECORContent/ProjectBP/Main/AE_MyCharacter.AE_MyCharacter_C|GetIsObjectHighlighted (stale EventBeginPlay _asae_my_character))
      (Default|GetBestInteractable (stale EventBeginPlay _asae_my_character))
      (else
        (bind _output_get_2 (Variables|Default|SetRenderCustomDepth false))
        (Rendering|SetRenderCustomDepth (Variables|Default|GetSkeletalMesh) _output_get_2)
        (Rendering|SetRenderCustomDepth (Variables|Default|GetStaticMesh) _output_get_2)
        (goto _label)))))

(event EventBeginPlay
  (bind _asae_my_character (Utilities|Casting|CastToAE_MyCharacter (Game|GetPlayerCharacter 0)))
  (CallFunction|UpdatePostProcessRender))

(fn ConstructionScript)