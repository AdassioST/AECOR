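; BP_CharacterRecorder is a scene-capture character stand-in that mirrors equipped gear on its Mesh2P.
; On BeginPlay it passes itself to the player's AE_MyCharacter through PassReferenceMessage.
; EquipItem switches on item slot, replaces that slot's actor with a spawned ItemClass, snaps it to its AttachPoint socket and disables collision.
; UnequipItem destroys the slot's actor, without the validity check used when equipping.
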(event EventBeginPlay
  (bind _asae_my_character (Utilities|Casting|CastToAE_MyCharacter (Game|GetPlayerCharacter 0)))
  (Class|BPIRecorderComm|PassReference(Message) _asae_my_character self))

(event EventEquipItem
  (params (ItemInfo :type F%20Item%20Info%20Structure))
  (CallFunction|AttachEquipment ItemInfo))

(event EventUnequipItem
  (params (ItemInfo :type F%20Item%20Info%20Structure))
  (CallFunction|UnattachEquipment ItemInfo))

(fn ConstructionScript)

(fn AttachEquipment
  (params (ItemInfo :type F%20Item%20Info%20Structure))
  (bind (_isitemconsumable _isitemequipable _itemclass _itemslot) (Utilities|Struct|BreakF_ItemInfo ItemInfo))
  (switch Utilities|FlowControl|Switch|SwitchonE_SlotType _itemslot
    (:NewEnumerator1
      ;[0 0.4104 0.4719] Exosuit
      (Utilities|IsValid (Variables|EquipmentSlotItems|GetExosuitItem)
        (:Is%20Valid
          (Actor|DestroyActor (Variables|EquipmentSlotItems|GetExosuitItem)))
        (:Is%20Not%20Valid
          _))
      (bind _returnvalue (Game|SpawnActorfromClass _itemclass (Transformation|GetActorTransform) "AlwaysSpawn" 0 0))
      (bind _output_get (Variables|EquipmentSlotItems|SetExosuitItem _returnvalue))
      (bind _asbp_base_equipment (Utilities|Casting|CastToBP_BaseEquipment _output_get))
      (Transformation|AttachComponentToComponent _asbp_base_equipment (Variables|Default|GetMesh2P) (Variables|/Game/AECORContent/ProjectBP/Environment/Interactables/Items/Equipment/BP_BaseEquipment.BP_BaseEquipment_C|GetAttachPoint _asbp_base_equipment) "SnapToTarget" "SnapToTarget" "SnapToTarget" true)
      (Collision|SetActorEnableCollision _asbp_base_equipment false))
    (:NewEnumerator2
      ;[0 0.4104 0.4719] Head Mounted Gadget
      (Utilities|IsValid (Variables|EquipmentSlotItems|GetHeadMGItem)
        (:Is%20Valid
          (Actor|DestroyActor (Variables|EquipmentSlotItems|GetHeadMGItem)))
        (:Is%20Not%20Valid
          _))
      (bind _returnvalue_2 (Game|SpawnActorfromClass _itemclass (Transformation|GetActorTransform) "AlwaysSpawn" 0 0))
      (bind _output_get_2 (Variables|EquipmentSlotItems|SetHeadMGItem _returnvalue_2))
      (bind _asbp_base_equipment_2 (Utilities|Casting|CastToBP_BaseEquipment _output_get_2))
      (Transformation|AttachComponentToComponent _asbp_base_equipment_2 (Variables|Default|GetMesh2P) (Variables|/Game/AECORContent/ProjectBP/Environment/Interactables/Items/Equipment/BP_BaseEquipment.BP_BaseEquipment_C|GetAttachPoint _asbp_base_equipment_2) "SnapToTarget" "SnapToTarget" "SnapToTarget" true)
      (Collision|SetActorEnableCollision _asbp_base_equipment_2 false))
    (:NewEnumerator3
      ;[0 0.4104 0.4719] Breathing System
      (Utilities|IsValid (Variables|EquipmentSlotItems|GetBreathingItem)
        (:Is%20Valid
          (Actor|DestroyActor (Variables|EquipmentSlotItems|GetBreathingItem)))
        (:Is%20Not%20Valid
          _))
      (bind _returnvalue_3 (Game|SpawnActorfromClass _itemclass (Transformation|GetActorTransform) "AlwaysSpawn" 0 0))
      (bind _output_get_3 (Variables|EquipmentSlotItems|SetBreathingItem _returnvalue_3))
      (bind _asbp_base_equipment_3 (Utilities|Casting|CastToBP_BaseEquipment _output_get_3))
      (Transformation|AttachComponentToComponent _asbp_base_equipment_3 (Variables|Default|GetMesh2P) (Variables|/Game/AECORContent/ProjectBP/Environment/Interactables/Items/Equipment/BP_BaseEquipment.BP_BaseEquipment_C|GetAttachPoint _asbp_base_equipment_3) "SnapToTarget" "SnapToTarget" "SnapToTarget" true)
      (Collision|SetActorEnableCollision _asbp_base_equipment_3 false))
    (:NewEnumerator4
      ;[0 0.4104 0.4719] Orientation Device
      (Utilities|IsValid (Variables|EquipmentSlotItems|GetOrientationItem)
        (:Is%20Valid
          (Actor|DestroyActor (Variables|EquipmentSlotItems|GetOrientationItem)))
        (:Is%20Not%20Valid
          _))
      (bind _returnvalue_4 (Game|SpawnActorfromClass _itemclass (Transformation|GetActorTransform) "AlwaysSpawn" 0 0))
      (bind _output_get_4 (Variables|EquipmentSlotItems|SetOrientationItem _returnvalue_4))
      (bind _asbp_base_equipment_4 (Utilities|Casting|CastToBP_BaseEquipment _output_get_4))
      (Transformation|AttachComponentToComponent _asbp_base_equipment_4 (Variables|Default|GetMesh2P) (Variables|/Game/AECORContent/ProjectBP/Environment/Interactables/Items/Equipment/BP_BaseEquipment.BP_BaseEquipment_C|GetAttachPoint _asbp_base_equipment_4) "SnapToTarget" "SnapToTarget" "SnapToTarget" true)
      (Collision|SetActorEnableCollision _asbp_base_equipment_4 false))
    (:NewEnumerator6
      ;[0 0.4104 0.4719] Utility Device
      (Utilities|IsValid (Variables|EquipmentSlotItems|GetUtilityItem)
        (:Is%20Valid
          (Actor|DestroyActor (Variables|EquipmentSlotItems|GetUtilityItem)))
        (:Is%20Not%20Valid
          _))
      (bind _returnvalue_5 (Game|SpawnActorfromClass _itemclass (Transformation|GetActorTransform) "AlwaysSpawn" 0 0))
      (bind _output_get_5 (Variables|EquipmentSlotItems|SetUtilityItem _returnvalue_5))
      (bind _asbp_base_equipment_5 (Utilities|Casting|CastToBP_BaseEquipment _output_get_5))
      (Transformation|AttachComponentToComponent _asbp_base_equipment_5 (Variables|Default|GetMesh2P) (Variables|/Game/AECORContent/ProjectBP/Environment/Interactables/Items/Equipment/BP_BaseEquipment.BP_BaseEquipment_C|GetAttachPoint _asbp_base_equipment_5) "SnapToTarget" "SnapToTarget" "SnapToTarget" true)
      (Collision|SetActorEnableCollision _asbp_base_equipment_5 false))
    (:NewEnumerator5
      ;[0 0.4104 0.4719] Fins Augmentation
      (Utilities|IsValid (Variables|EquipmentSlotItems|GetFinsItem)
        (:Is%20Valid
          (Actor|DestroyActor (Variables|EquipmentSlotItems|GetFinsItem)))
        (:Is%20Not%20Valid
          _))
      (bind _returnvalue_6 (Game|SpawnActorfromClass _itemclass (Transformation|GetActorTransform) "AlwaysSpawn" 0 0))
      (bind _output_get_6 (Variables|EquipmentSlotItems|SetFinsItem _returnvalue_6))
      (bind _asbp_base_equipment_6 (Utilities|Casting|CastToBP_BaseEquipment _output_get_6))
      (Transformation|AttachComponentToComponent _asbp_base_equipment_6 (Variables|Default|GetMesh2P) (Variables|/Game/AECORContent/ProjectBP/Environment/Interactables/Items/Equipment/BP_BaseEquipment.BP_BaseEquipment_C|GetAttachPoint _asbp_base_equipment_6) "SnapToTarget" "SnapToTarget" "SnapToTarget" true)
      (Collision|SetActorEnableCollision _asbp_base_equipment_6 false))
    (:NewEnumerator10
      ;[0 0.4104 0.4719] Arms Module
      (Utilities|IsValid (Variables|EquipmentSlotItems|GetArmsItem)
        (:Is%20Valid
          (Actor|DestroyActor (Variables|EquipmentSlotItems|GetArmsItem)))
        (:Is%20Not%20Valid
          _))
      (bind _returnvalue_7 (Game|SpawnActorfromClass _itemclass (Transformation|GetActorTransform) "AlwaysSpawn" 0 0))
      (bind _output_get_7 (Variables|EquipmentSlotItems|SetArmsItem _returnvalue_7))
      (bind _asbp_base_equipment_7 (Utilities|Casting|CastToBP_BaseEquipment _output_get_7))
      (Transformation|AttachComponentToComponent _asbp_base_equipment_7 (Variables|Default|GetMesh2P) (Variables|/Game/AECORContent/ProjectBP/Environment/Interactables/Items/Equipment/BP_BaseEquipment.BP_BaseEquipment_C|GetAttachPoint _asbp_base_equipment_7) "SnapToTarget" "SnapToTarget" "SnapToTarget" true)
      (Collision|SetActorEnableCollision _asbp_base_equipment_7 false))
    (:NewEnumerator9
      ;[0 0.4104 0.4719] Back Module
      (Utilities|IsValid (Variables|EquipmentSlotItems|GetBackItem)
        (:Is%20Valid
          (Actor|DestroyActor (Variables|EquipmentSlotItems|GetBackItem)))
        (:Is%20Not%20Valid
          _))
      (bind _returnvalue_8 (Game|SpawnActorfromClass _itemclass (Transformation|GetActorTransform) "AlwaysSpawn" 0 0))
      (bind _output_get_8 (Variables|EquipmentSlotItems|SetBackItem _returnvalue_8))
      (bind _asbp_base_equipment_8 (Utilities|Casting|CastToBP_BaseEquipment _output_get_8))
      (Transformation|AttachComponentToComponent _asbp_base_equipment_8 (Variables|Default|GetMesh2P) (Variables|/Game/AECORContent/ProjectBP/Environment/Interactables/Items/Equipment/BP_BaseEquipment.BP_BaseEquipment_C|GetAttachPoint _asbp_base_equipment_8) "SnapToTarget" "SnapToTarget" "SnapToTarget" true)
      (Collision|SetActorEnableCollision _asbp_base_equipment_8 false))
    (:NewEnumerator7
      ;[0 0.4104 0.4719] Self Defense Module
      (Utilities|IsValid (Variables|EquipmentSlotItems|GetSelfDefenseItem)
        (:Is%20Valid
          (Actor|DestroyActor (Variables|EquipmentSlotItems|GetSelfDefenseItem)))
        (:Is%20Not%20Valid
          _))
      (bind _returnvalue_9 (Game|SpawnActorfromClass _itemclass (Transformation|GetActorTransform) "AlwaysSpawn" 0 0))
      (bind _output_get_9 (Variables|EquipmentSlotItems|SetSelfDefenseItem _returnvalue_9))
      (bind _asbp_base_equipment_9 (Utilities|Casting|CastToBP_BaseEquipment _output_get_9))
      (Transformation|AttachComponentToComponent _asbp_base_equipment_9 (Variables|Default|GetMesh2P) (Variables|/Game/AECORContent/ProjectBP/Environment/Interactables/Items/Equipment/BP_BaseEquipment.BP_BaseEquipment_C|GetAttachPoint _asbp_base_equipment_9) "SnapToTarget" "SnapToTarget" "SnapToTarget" true)
      (Collision|SetActorEnableCollision _asbp_base_equipment_9 false))
    (:NewEnumerator8
      ;[0 0.4104 0.4719] SPHERE Companion
      (Utilities|IsValid (Variables|EquipmentSlotItems|GetSphereItem)
        (:Is%20Valid
          (Actor|DestroyActor (Variables|EquipmentSlotItems|GetSphereItem)))
        (:Is%20Not%20Valid
          _))
      (bind _returnvalue_10 (Game|SpawnActorfromClass _itemclass (Transformation|GetActorTransform) "AlwaysSpawn" 0 0))
      (bind _output_get_10 (Variables|EquipmentSlotItems|SetSphereItem _returnvalue_10))
      (bind _asbp_base_equipment_10 (Utilities|Casting|CastToBP_BaseEquipment _output_get_10))
      (Transformation|AttachComponentToComponent _asbp_base_equipment_10 (Variables|Default|GetMesh2P) (Variables|/Game/AECORContent/ProjectBP/Environment/Interactables/Items/Equipment/BP_BaseEquipment.BP_BaseEquipment_C|GetAttachPoint _asbp_base_equipment_10) "SnapToTarget" "SnapToTarget" "SnapToTarget" true)
      (Collision|SetActorEnableCollision _asbp_base_equipment_10 false))))

(fn UnattachEquipment
  (params (ItemInfo :type F%20Item%20Info%20Structure))
  (switch Utilities|FlowControl|Switch|SwitchonE_SlotType (.ItemSlot (Utilities|Struct|BreakF_ItemInfo ItemInfo))
    (:NewEnumerator1
      ;[0 0.4082 0.4802] Exosuit
      (Actor|DestroyActor (Variables|EquipmentSlotItems|GetExosuitItem)))
    (:NewEnumerator2
      ;[0 0.4082 0.4802] Head Mounted Gadget
      (Actor|DestroyActor (Variables|EquipmentSlotItems|GetHeadMGItem)))
    (:NewEnumerator3
      ;[0 0.4082 0.4802] Breathing System
      (Actor|DestroyActor (Variables|EquipmentSlotItems|GetBreathingItem)))
    (:NewEnumerator4
      ;[0 0.4082 0.4802] Orientation Device
      (Actor|DestroyActor (Variables|EquipmentSlotItems|GetOrientationItem)))
    (:NewEnumerator6
      ;[0 0.4082 0.4802] Utility Device
      (Actor|DestroyActor (Variables|EquipmentSlotItems|GetUtilityItem)))
    (:NewEnumerator5
      ;[0 0.4082 0.4802] Fins Augmentation
      (Actor|DestroyActor (Variables|EquipmentSlotItems|GetFinsItem)))
    (:NewEnumerator10
      ;[0 0.4082 0.4802] Arms Module
      (Actor|DestroyActor (Variables|EquipmentSlotItems|GetArmsItem)))
    (:NewEnumerator9
      ;[0 0.4082 0.4802] Back Module
      (Actor|DestroyActor (Variables|EquipmentSlotItems|GetBackItem)))
    (:NewEnumerator7
      ;[0 0.4082 0.4802] Self Defense Module
      (Actor|DestroyActor (Variables|EquipmentSlotItems|GetSelfDefenseItem)))
    (:NewEnumerator8
      ;[0 0.4082 0.4802] SPHERE Companion
      (Actor|DestroyActor (Variables|EquipmentSlotItems|GetSphereItem)))))