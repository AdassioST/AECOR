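; Base vehicle Blueprint with physics-driven throttle, three-axis rotation and collision damage, tuned through VehicleInfo.
; Input axes apply torque around the mesh's axes, while Tick counters angular velocity to damp spin.
; Throttle ramps while held and eases toward zero, blending velocity along the negative right vector, the mesh's travel axis.
; Hits, throttled by a delayed DoOnce, subtract health from world-X speed; DestroyVehicle only prints a warning.
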(event OnComponentHit(VehicleMesh)
  (params (HitComponent :type Primitive%20Component%20Object%20Reference) (OtherActor :type Actor%20Object%20Reference) (OtherComp :type Primitive%20Component%20Object%20Reference) (NormalImpulse :type Vector :default "0, 0, 0") (Hit :type Hit%20Result%20Structure%20%28by%20ref%29))
  (Utilities|FlowControl|DoOnce false :!label _label
    (:Completed
      (bind _returnvalue (Physics|GetPhysicsLinearVelocity (Variables|Default|GetVehicleMesh) "None"))
      (bind _output_get (Variables|Default|SetVehicleHealth (Math|Float|Clamp(Float) (- (Variables|Default|GetVehicleHealth) (Math|Float|Absolute(Float) (/ (.X (Math|Vector|BreakVector _returnvalue)) 1e+02))) 0.0 (Variables|Default|GetMaxVehicleHealth))))
      (if (not (<= (Variables|Default|GetVehicleHealth) 0.0))
        (Development|PrintString (Utilities|String|ToString(Float) _output_get) true true "(R=0.962563,G=1.000000,B=0.000000,A=1.000000)")
        (else
          (CallFunction|DestroyVehicle)))
      (Utilities|FlowControl|Delay 0.5)
      (goto _label Reset))))

(event Collision|EventActorBeginOverlap
  (params (OtherActor :type Actor%20Object%20Reference)))

(event EventTick
  (params (DeltaSeconds :type Float%20%28single-precision%29))
  (bind _vehiclemesh (Variables|Default|GetVehicleMesh))
  ;[0.3134 1 0.1362] Correct Movement and Add Throttle
  (CallFunction|ThrottleInput)
  (Class|PrimitiveComponent|AddTorqueinDegrees _vehiclemesh (/ (Math|Vector|NegateVector (Physics|GetPhysicsAngularVelocityinDegrees (Variables|Default|GetVehicleMesh) "None")) 0.5) "None" true)
  (Physics|AddForce _vehiclemesh "0, 0,0.000000" "None" true)
  (CallFunction|CalculateVehicleSpeed))

(event Input|ActionEvents|InputActionVehicleThrottleDown
  (params (Key :type Key%20Structure))
  (:Pressed
    (Variables|Default|SetThrottleDown true))
  (:Released
    (Variables|Default|SetThrottleDown false)))

(event Input|ActionEvents|InputActionVehicleThrottleUp
  (params (Key :type Key%20Structure))
  (:Pressed
    (Variables|Default|SetThrottleUp true))
  (:Released
    (Variables|Default|SetThrottleUp false)))

(event Input|AxisEvents|InputAxisMoveRight
  (params (AxisValue :type Float%20%28single-precision%29))
  ;[0 1 0.6115] Axis Movement
  (Class|PrimitiveComponent|AddTorqueinDegrees (Variables|Default|GetVehicleMesh) (Math|Vector|Lerp(Vector) "0, 0, 0" (* (Math|Vector|GetUpVector (Variables|Default|GetVehicleMesh)) (* AxisValue (.VehicleTractionControl (Utilities|Struct|BreakF_VehicleInfo (Variables|Default|GetVehicleInfo))))) 0.1) "None" true))

(event Input|AxisEvents|InputAxisMoveForward
  (params (AxisValue :type Float%20%28single-precision%29))
  ;[0 1 0.6115] Axis Movement
  (Class|PrimitiveComponent|AddTorqueinDegrees (Variables|Default|GetVehicleMesh) (Math|Vector|Lerp(Vector) "0, 0, 0" (* (Math|Vector|GetForwardVector (Variables|Default|GetVehicleMesh)) (* (* AxisValue -1.0) (.VehicleTractionControl (Utilities|Struct|BreakF_VehicleInfo (Variables|Default|GetVehicleInfo))))) 0.1) "None" true))

(event Input|AxisEvents|InputAxisVehicleRoll
  (params (AxisValue :type Float%20%28single-precision%29))
  (bind _vehicleinfo (Variables|Default|GetVehicleInfo))
  (bind (_vehiclemaxthrottle _vehicletractioncontrol _vehiclemaxspeed _canvehicleroll) (Utilities|Struct|BreakF_VehicleInfo _vehicleinfo))
  ;[0 1 0.6115] Axis Movement
  (if _canvehicleroll
    (Class|PrimitiveComponent|AddTorqueinDegrees (Variables|Default|GetVehicleMesh) (Math|Vector|Lerp(Vector) "0, 0, 0" (* (Math|Vector|GetRightVector (Variables|Default|GetVehicleMesh)) (* AxisValue _vehicletractioncontrol)) 0.1) "None" true)))

(fn ConstructionScript)

(fn ThrottleInput
  (bind _vehicleinfo (Variables|Default|GetVehicleInfo))
  (bind _vehiclemaxthrottle (Utilities|Struct|BreakF_VehicleInfo _vehicleinfo))
  (bind _returnvalue (* _vehiclemaxthrottle -1.0))
  (if (Variables|Default|GetThrottleUp)
    (Variables|Default|SetVehicleThrottleAmount (Math|Float|Clamp(Float) (+ (Variables|Default|GetVehicleThrottleAmount) (Variables|Default|GetThrottleRecoveryRate)) _returnvalue _vehiclemaxthrottle))
    (elif (Variables|Default|GetThrottleDown)
      (Variables|Default|SetVehicleThrottleAmount (Math|Float|Clamp(Float) (- (Variables|Default|GetVehicleThrottleAmount) (Variables|Default|GetThrottleRecoveryRate)) _returnvalue _vehiclemaxthrottle))
      (else
        (CallFunction|RegulateThrottletoZero)))))

(fn CalculateVehicleSpeed
  (bind _vehiclemesh (Variables|Default|GetVehicleMesh))
  (bind _vehicleinfo (Variables|Default|GetVehicleInfo))
  (bind _vehiclemaxspeed (Utilities|Struct|BreakF_VehicleInfo _vehicleinfo))
  (bind _returnvalue (Physics|GetPhysicsLinearVelocity _vehiclemesh "None"))
  (Physics|SetPhysicsLinearVelocity (Variables|Default|GetVehicleMesh) (Math|Vector|Lerp(Vector) _returnvalue (* (Math|Vector|GetRightVector _vehiclemesh) (* (Math|Float|Clamp(Float) (* (Variables|Default|GetVehicleThrottleAmount) 2.5e+02) (* _vehiclemaxspeed -0.25) _vehiclemaxspeed) -1.0)) 0.01) false "None"))

(fn RegulateThrottletoZero
  (if (> (Variables|Default|GetVehicleThrottleAmount) 0.0)
    (Variables|Default|SetVehicleThrottleAmount (- (Variables|Default|GetVehicleThrottleAmount) (* (Variables|Default|GetThrottleRecoveryRate) 0.5)))
    (elif (< (Variables|Default|GetVehicleThrottleAmount) 0.0)
      (Variables|Default|SetVehicleThrottleAmount (+ (Variables|Default|GetVehicleThrottleAmount) (* (Variables|Default|GetThrottleRecoveryRate) 0.5))))))

(fn DestroyVehicle
  (Development|PrintString "Vehicle health is critical, it should be destroyed" true true "(R=1.000000,G=0.000000,B=0.028684,A=1.000000)"))