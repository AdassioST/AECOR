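; Test actor that ropes two actors together with a breakable physics constraint and a visual cable, likely for ocean buoyancy examples.
; Hook runs on construction and BeginPlay, constraining both root components and scaling linear limits, cable length and material tiling from the distance between reference points.
; When the constraint breaks, it reattaches the cable end to a spawned hidden BP_BuoyantActor that blocks only WorldStatic, leaving the loose end buoyant.
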(event OnConstraintBroken(PhysicsConstraint)
  (params (ConstraintIndex :type Integer))
  (bind _cable (Variables|Default|GetCable))
  (bind _returnvalue (Game|SpawnActorfromClass "/Game/Z_OceanAssets/Ocean/BP_BuoyantActor.BP_BuoyantActor_C" (Transformation|GetActorTransform (Class|CableComponent|GetAttachedActor _cable)) "AdjustIfPossibleButAlwaysSpawn" 0 1025.0 1025.0 1.0 1.0 false 1e+03 1e+01 (Utilities|Array|MakeArray "0, 0, 0") 0))
  (Rendering|SetActorHiddenInGame _returnvalue true)
  (Collision|SetCollisionResponsetoAllChannels (Variables|/Script/Engine.StaticMeshActor|GetStaticMeshComponent _returnvalue) "ECR_Ignore")
  (Collision|SetCollisionResponsetoChannel (Variables|/Script/Engine.StaticMeshActor|GetStaticMeshComponent _returnvalue) "ECC_WorldStatic" "ECR_Block")
  (Class|CableComponent|SetAttachEndto _cable _returnvalue "None" "None")
  (Variables|/Script/CableComponent.CableComponent|SetEndLocation _cable "0, 0, 0"))

(event Custom|Hook
  (bind _actor1 (Variables|Default|GetActor1))
  (bind _actor2 (Variables|Default|GetActor2))
  (bind _cable (Variables|Default|GetCable))
  (bind _physicsconstraint (Variables|Default|GetPhysicsConstraint))
  (bind _distance (Variables|Default|GetDistance))
  (bind _refpos1 (Variables|Default|GetRefPos1))
  (bind _refpos2 (Variables|Default|GetRefPos2))
  (bind _returnvalue (Transformation|GetActorTransform _actor2))
  (bind _returnvalue_2 (Transformation|GetActorTransform _actor1))
  (bind _returnvalue_3 (Math|Transform|TransformLocation _returnvalue _refpos2))
  (bind _returnvalue_4 (Math|Transform|TransformLocation _returnvalue_2 _refpos1))
  (bind _returnvalue_5 (- _returnvalue_4 _returnvalue_3))
  (bind _returnvalue_6 (Math|Vector|VectorLength _returnvalue_5))
  (bind _returnvalue_7 (/ _returnvalue_6 3.0))
  (bind _returnvalue_8 (/ _returnvalue_6 4.0))
  (bind _returnvalue_9 (+ _distance _returnvalue_7))
  (Utilities|IsValid (Variables|Default|GetActor1)
    (:Is%20Valid
      (Utilities|IsValid (Variables|Default|GetActor2)
        (:Is%20Valid
          (bind _asprimitive_component (Utilities|Casting|CastToPrimitiveComponent (VehicleSound|GetRootComponent (Variables|Default|GetActor1))))
          (bind _asprimitive_component_2 (Utilities|Casting|CastToPrimitiveComponent (VehicleSound|GetRootComponent (Variables|Default|GetActor2))))
          (if (and (Utilities|IsValid (Variables|Default|GetActor1)) (Utilities|IsValid (Variables|Default|GetActor2)))
            (Class|PhysicsConstraintComponent|SetConstrainedComponents (Variables|Default|GetPhysicsConstraint) _asprimitive_component "None" _asprimitive_component_2 "None")
            (Class|PhysicsConstraintComponent|SetConstraintReferencePosition _physicsconstraint "Frame1" (Variables|Default|GetRefPos1))
            (Class|PhysicsConstraintComponent|SetConstraintReferencePosition _physicsconstraint "Frame2" (Variables|Default|GetRefPos2))
            (Class|PhysicsConstraintComponent|SetLinearXLimit _physicsconstraint "LCM_Limited" _returnvalue_9)
            (Class|PhysicsConstraintComponent|SetLinearYLimit _physicsconstraint "LCM_Limited" _returnvalue_9)
            (Class|PhysicsConstraintComponent|SetLinearZLimit _physicsconstraint "LCM_Limited" _returnvalue_9)
            (Class|CableComponent|SetAttachEndto _cable (Variables|Default|GetActor2) "None" "None")
            (Variables|/Script/CableComponent.CableComponent|SetEndLocation _cable (Variables|Default|GetRefPos2))
            (Variables|/Script/CableComponent.CableComponent|SetCableLength _cable (+ (* _returnvalue_8 0.9) (Variables|Default|GetCableLength)))
            (Variables|/Script/CableComponent.CableComponent|SetCableWidth _cable (Variables|Default|GetCableWidth))
            (Variables|/Script/CableComponent.CableComponent|SetTileMaterial _cable (* _returnvalue_8 0.05))))))))

(event EventBeginPlay
  (CallFunction|Hook))

(fn ConstructionScript
  (CallFunction|Hook))