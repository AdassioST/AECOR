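; BP_Wake is a short-lived ocean foam wake actor that expands and fades out after it spawns.
; The construction script creates a dynamic M_Wake material instance on a plane mesh and sets a fallback lifespan.
; Tick grows Radius and lowers Opacity at constant rates, feeding both to the material so the animation is shader-driven.
; The actor destroys itself once Opacity reaches zero.
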(event EventTick
  (params (DeltaSeconds :type Float%20%28single-precision%29))
  (bind _m_inst (Variables|Default|GetM_Inst))
  (bind _output_get (Variables|Default|SetRadius (+ (Variables|Default|GetRadius) (* DeltaSeconds 2.5e+02))))
  (Rendering|Material|SetScalarParameterValue _m_inst "Radius" _output_get :!class /Script/Engine.MaterialInstanceDynamic)
  (bind _output_get_2 (Variables|Default|SetOpacity (- (Variables|Default|GetOpacity) (* DeltaSeconds 0.1))))
  (Rendering|Material|SetScalarParameterValue _m_inst "Opacity" _output_get_2 :!class /Script/Engine.MaterialInstanceDynamic)
  (if (<= (Variables|Default|GetOpacity) 0.0)
    (Actor|DestroyActor)))

(fn ConstructionScript
  (bind _returnvalue (Rendering|Material|CreateDynamicMaterialInstance (Variables|Default|GetSM_SplinePlaneMesh) 0 "/Game/Z_OceanAssets/Ocean/FoamWakes/M_Wake.M_Wake" "None" :!class /Script/Engine.PrimitiveComponent))
  (Variables|Default|SetM_Inst _returnvalue)
  (Actor|SetLifeSpan 15.0))