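; Ocean manager that computes Gerstner wave height on the CPU and applies point buoyancy forces to physics components.
; Construction reads global settings and wave sets from material parameter collection values; BeginPlay reloads only the wave sets.
; Each set averages eight Gerstner waves, and an optional second set is averaged with the first.
; ProcessBuoyancy samples height at a point, pushing up underwater or down above it, scaled by clamped squared depth over thickness.
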(event EventBeginPlay
  ;[1 1 1] Re-Run Initialization on Begin Play (Required for MaterialParameterCollection's)
  (Utilities|FlowControl|Sequence
    (:then_0
      (CallFunction|InitWaveSet1))
    (:then_1
      (if (Variables|Default|GetUse%20Wave%20Set%2002)
        (CallFunction|InitWaveSet2)))))

(fn ConstructionScript
  ;[1 1 1] Initialize Wave Parameters & Sets
  (CallFunction|InitGlobalParameters)
  (Utilities|FlowControl|Sequence
    (:then_0
      (CallFunction|InitWaveSet1))
    (:then_1
      (if (Variables|Default|GetUse%20Wave%20Set%2002)
        (CallFunction|InitWaveSet2)))))

(fn CalculateGerstnerWave
  (params (World%20Position :type Vector) (Direction%20V2 :type Vector) (Wave%20Rotation :type Float%20%28single-precision%29) (Wave%20Length :type Float%20%28single-precision%29) (Wave%20Amplitude :type Float%20%28single-precision%29) (Wave%20Steepness :type Float%20%28single-precision%29) (Time :type Float%20%28single-precision%29))
  (bind _returnvalue (Math|Float|MultiplybyPi 2.0))
  (bind (_x _y) (Math|Vector|BreakVector World%20Position))
  (bind _returnvalue_2 (Math|Float|MultiplybyPi 2.0))
  (bind _returnvalue_3 (Math|Float|MapRangeUnclamped Wave%20Rotation 0.0 1.0 0.0 3.6e+02))
  (bind _returnvalue_4 (Math|Vector|RotateVectorAroundAxis Direction%20V2 _returnvalue_3 "0, 0, 0"))
  (bind _returnvalue_5 (/ _returnvalue Wave%20Length))
  (bind _returnvalue_6 (Math|Vector|MakeVector _x _y 0.0))
  (bind _returnvalue_7 (Math|Vector|Normalize _returnvalue_4))
  (bind _returnvalue_8 (Math|Vector|DotProduct _returnvalue_6 _returnvalue_7))
  (bind (_x_2 _y_2) (Math|Vector|BreakVector _returnvalue_7))
  (bind _returnvalue_9 (* _returnvalue_8 _returnvalue_5))
  (bind _returnvalue_10 (+ _returnvalue_9 Time))
  (bind _returnvalue_11 (/ _returnvalue_10 _returnvalue_2))
  (bind _returnvalue_12 (Math|Trig|Cos(Radians) _returnvalue_11))
  (bind _returnvalue_13 (* _returnvalue_12 Wave%20Steepness))
  (bind _returnvalue_14 (* _returnvalue_13 Wave%20Amplitude))
  ;[1 1 1] The Gerstner Wave Equation (See documentation for more info)
  (return (Math|Vector|MakeVector (* _x_2 _returnvalue_14) (* _y_2 _returnvalue_14) (* (Math|Trig|Sin(Radians) _returnvalue_11) Wave%20Amplitude))))

(fn CreateWaveSet
  (params (World%20Position :type Vector) (Wave%20Direction%20V2 :type Vector) (Time :type Float%20%28single-precision%29) (Global%20Wave%20Parameters :type Wave%20Parameters%20Structure) (Wave%20Set%20Parameters :type Wave%20Set%20Structure))
  (bind (_wave01 _wave02 _wave03 _wave04 _wave05 _wave06 _wave07 _wave08) (Utilities|Struct|BreakWaveSet Wave%20Set%20Parameters))
  (bind (_rotation _length _amplitude _steepness) (Utilities|Struct|BreakWaveParameters Global%20Wave%20Parameters))
  (bind (_rotation_2 _length_2 _amplitude_2 _steepness_2) (Utilities|Struct|BreakWaveParameters _wave01))
  (bind (_rotation_3 _length_3 _amplitude_3 _steepness_3) (Utilities|Struct|BreakWaveParameters _wave02))
  (bind (_rotation_4 _length_4 _amplitude_4 _steepness_4) (Utilities|Struct|BreakWaveParameters _wave03))
  (bind (_rotation_5 _length_5 _amplitude_5 _steepness_5) (Utilities|Struct|BreakWaveParameters _wave04))
  (bind (_rotation_6 _length_6 _amplitude_6 _steepness_6) (Utilities|Struct|BreakWaveParameters _wave05))
  (bind (_rotation_7 _length_7 _amplitude_7 _steepness_7) (Utilities|Struct|BreakWaveParameters _wave06))
  (bind (_rotation_8 _length_8 _amplitude_8 _steepness_8) (Utilities|Struct|BreakWaveParameters _wave07))
  (bind (_rotation_9 _length_9 _amplitude_9 _steepness_9) (Utilities|Struct|BreakWaveParameters _wave08))
  ;[1 1 1] Create a Wave Set from the Given Parameters
  (return (/ (+ (CallFunction|CalculateGerstnerWave World%20Position Wave%20Direction%20V2 (+ _rotation _rotation_2) (* _length _length_2) (* _amplitude _amplitude_2) (* _steepness _steepness_2) Time) (CallFunction|CalculateGerstnerWave World%20Position Wave%20Direction%20V2 (+ _rotation _rotation_3) (* _length _length_3) (* _amplitude _amplitude_3) (* _steepness _steepness_3) Time) (CallFunction|CalculateGerstnerWave World%20Position Wave%20Direction%20V2 (+ _rotation _rotation_4) (* _length _length_4) (* _amplitude _amplitude_4) (* _steepness _steepness_4) Time) (CallFunction|CalculateGerstnerWave World%20Position Wave%20Direction%20V2 (+ _rotation _rotation_5) (* _length _length_5) (* _amplitude _amplitude_5) (* _steepness _steepness_5) Time) (CallFunction|CalculateGerstnerWave World%20Position Wave%20Direction%20V2 (+ _rotation _rotation_6) (* _length _length_6) (* _amplitude _amplitude_6) (* _steepness _steepness_6) Time) (CallFunction|CalculateGerstnerWave World%20Position Wave%20Direction%20V2 (+ _rotation _rotation_7) (* _length _length_7) (* _amplitude _amplitude_7) (* _steepness _steepness_7) Time) (CallFunction|CalculateGerstnerWave World%20Position Wave%20Direction%20V2 (+ _rotation _rotation_8) (* _length _length_8) (* _amplitude _amplitude_8) (* _steepness _steepness_8) Time) (CallFunction|CalculateGerstnerWave World%20Position Wave%20Direction%20V2 (+ _rotation _rotation_9) (* _length _length_9) (* _amplitude _amplitude_9) (* _steepness _steepness_9) Time)) 8.0)))

(fn InitWaveSet1
  (Utilities|FlowControl|Sequence
    (:then_0
      ;[1 1 1] Retrieve The Parameters for the Wave Set from the MPC
      (Utilities|FlowControl|Sequence
        (:then_0
          (bind _returnvalue (Rendering|Material|GetVectorParameterValue 0 "Set01Wave01" :!class /Script/Engine.KismetMaterialLibrary))
          (Variables|WaveSet1|SetSet01Wave01 (Utilities|Struct|MakeWaveParameters (.r _returnvalue) (.g _returnvalue) (.b _returnvalue) (.a _returnvalue) 1.0)))
        (:then_1
          (bind _returnvalue_2 (Rendering|Material|GetVectorParameterValue 0 "Set01Wave02" :!class /Script/Engine.KismetMaterialLibrary))
          (Variables|WaveSet1|SetSet01Wave02 (Utilities|Struct|MakeWaveParameters (.r _returnvalue_2) (.g _returnvalue_2) (.b _returnvalue_2) (.a _returnvalue_2) 1.0)))
        (:then_2
          (bind _returnvalue_3 (Rendering|Material|GetVectorParameterValue 0 "Set01Wave03" :!class /Script/Engine.KismetMaterialLibrary))
          (Variables|WaveSet1|SetSet01Wave03 (Utilities|Struct|MakeWaveParameters (.r _returnvalue_3) (.g _returnvalue_3) (.b _returnvalue_3) (.a _returnvalue_3) 1.0)))
        (:then_3
          (bind _returnvalue_4 (Rendering|Material|GetVectorParameterValue 0 "Set01Wave04" :!class /Script/Engine.KismetMaterialLibrary))
          (Variables|WaveSet1|SetSet01Wave04 (Utilities|Struct|MakeWaveParameters (.r _returnvalue_4) (.g _returnvalue_4) (.b _returnvalue_4) (.a _returnvalue_4) 1.0)))
        (:then_4
          (bind _returnvalue_5 (Rendering|Material|GetVectorParameterValue 0 "Set01Wave05" :!class /Script/Engine.KismetMaterialLibrary))
          (Variables|WaveSet1|SetSet01Wave05 (Utilities|Struct|MakeWaveParameters (.r _returnvalue_5) (.g _returnvalue_5) (.b _returnvalue_5) (.a _returnvalue_5) 1.0)))
        (:then_5
          (bind _returnvalue_6 (Rendering|Material|GetVectorParameterValue 0 "Set01Wave06" :!class /Script/Engine.KismetMaterialLibrary))
          (Variables|WaveSet1|SetSet01Wave06 (Utilities|Struct|MakeWaveParameters (.r _returnvalue_6) (.g _returnvalue_6) (.b _returnvalue_6) (.a _returnvalue_6) 1.0)))
        (:then_6
          (bind _returnvalue_7 (Rendering|Material|GetVectorParameterValue 0 "Set01Wave07" :!class /Script/Engine.KismetMaterialLibrary))
          (Variables|WaveSet1|SetSet01Wave07 (Utilities|Struct|MakeWaveParameters (.r _returnvalue_7) (.g _returnvalue_7) (.b _returnvalue_7) (.a _returnvalue_7) 1.0)))
        (:then_7
          (bind _returnvalue_8 (Rendering|Material|GetVectorParameterValue 0 "Set01Wave08" :!class /Script/Engine.KismetMaterialLibrary))
          (Variables|WaveSet1|SetSet01Wave08 (Utilities|Struct|MakeWaveParameters (.r _returnvalue_8) (.g _returnvalue_8) (.b _returnvalue_8) (.a _returnvalue_8) 1.0)))))
    (:then_1
      ;[1 1 1] Create the Wave Set Struct
      (Variables|Default|SetWave%20Set%2001 (Utilities|Struct|MakeWaveSet (Variables|WaveSet1|GetSet01Wave01) (Variables|WaveSet1|GetSet01Wave02) (Variables|WaveSet1|GetSet01Wave03) (Variables|WaveSet1|GetSet01Wave04) (Variables|WaveSet1|GetSet01Wave05) (Variables|WaveSet1|GetSet01Wave06) (Variables|WaveSet1|GetSet01Wave07) (Variables|WaveSet1|GetSet01Wave08))))))

(fn InitWaveSet2
  (Utilities|FlowControl|Sequence
    (:then_0
      ;[1 1 1] Retrieve The Parameters for the Wave Set from the MPC
      (Utilities|FlowControl|Sequence
        (:then_0
          (bind _returnvalue (Rendering|Material|GetVectorParameterValue 0 "Set02Wave01" :!class /Script/Engine.KismetMaterialLibrary))
          (Variables|WaveSet2|SetSet02Wave01 (Utilities|Struct|MakeWaveParameters (.r _returnvalue) (.g _returnvalue) (.b _returnvalue) (.a _returnvalue) 1.0)))
        (:then_1
          (bind _returnvalue_2 (Rendering|Material|GetVectorParameterValue 0 "Set02Wave02" :!class /Script/Engine.KismetMaterialLibrary))
          (Variables|WaveSet2|SetSet02Wave02 (Utilities|Struct|MakeWaveParameters (.r _returnvalue_2) (.g _returnvalue_2) (.b _returnvalue_2) (.a _returnvalue_2) 1.0)))
        (:then_2
          (bind _returnvalue_3 (Rendering|Material|GetVectorParameterValue 0 "Set02Wave03" :!class /Script/Engine.KismetMaterialLibrary))
          (Variables|WaveSet2|SetSet02Wave03 (Utilities|Struct|MakeWaveParameters (.r _returnvalue_3) (.g _returnvalue_3) (.b _returnvalue_3) (.a _returnvalue_3) 1.0)))
        (:then_3
          (bind _returnvalue_4 (Rendering|Material|GetVectorParameterValue 0 "Set02Wave04" :!class /Script/Engine.KismetMaterialLibrary))
          (Variables|WaveSet2|SetSet02Wave04 (Utilities|Struct|MakeWaveParameters (.r _returnvalue_4) (.g _returnvalue_4) (.b _returnvalue_4) (.a _returnvalue_4) 1.0)))
        (:then_4
          (bind _returnvalue_5 (Rendering|Material|GetVectorParameterValue 0 "Set02Wave05" :!class /Script/Engine.KismetMaterialLibrary))
          (Variables|WaveSet2|SetSet02Wave05 (Utilities|Struct|MakeWaveParameters (.r _returnvalue_5) (.g _returnvalue_5) (.b _returnvalue_5) (.a _returnvalue_5) 1.0)))
        (:then_5
          (bind _returnvalue_6 (Rendering|Material|GetVectorParameterValue 0 "Set02Wave06" :!class /Script/Engine.KismetMaterialLibrary))
          (Variables|WaveSet2|SetSet02Wave06 (Utilities|Struct|MakeWaveParameters (.r _returnvalue_6) (.g _returnvalue_6) (.b _returnvalue_6) (.a _returnvalue_6) 1.0)))
        (:then_6
          (bind _returnvalue_7 (Rendering|Material|GetVectorParameterValue 0 "Set02Wave07" :!class /Script/Engine.KismetMaterialLibrary))
          (Variables|WaveSet2|SetSet02Wave07 (Utilities|Struct|MakeWaveParameters (.r _returnvalue_7) (.g _returnvalue_7) (.b _returnvalue_7) (.a _returnvalue_7) 1.0)))
        (:then_7
          (bind _returnvalue_8 (Rendering|Material|GetVectorParameterValue 0 "Set02Wave08" :!class /Script/Engine.KismetMaterialLibrary))
          (Variables|WaveSet2|SetSet02Wave08 (Utilities|Struct|MakeWaveParameters (.r _returnvalue_8) (.g _returnvalue_8) (.b _returnvalue_8) (.a _returnvalue_8) 1.0)))))
    (:then_1
      ;[1 1 1] Create the Wave Set Struct
      (Variables|Default|SetWave%20Set%2002 (Utilities|Struct|MakeWaveSet (Variables|WaveSet2|GetSet02Wave01) (Variables|WaveSet2|GetSet02Wave02) (Variables|WaveSet2|GetSet02Wave03) (Variables|WaveSet2|GetSet02Wave04) (Variables|WaveSet2|GetSet02Wave05) (Variables|WaveSet2|GetSet02Wave06) (Variables|WaveSet2|GetSet02Wave07) (Variables|WaveSet2|GetSet02Wave08))))))

(fn GetWaveHeight
  (params (Location :type Vector) (Time :type Float%20%28single-precision%29))
  (bind _wave_direction_v2 (Variables|Default|GetWave%20Direction%20V2))
  (bind _global_wave_settings (Variables|Default|GetGlobal%20Wave%20Settings))
  ;[1 1 1] Create Wave Sets and Return Height at Point
  (LocalVariables|SetSum%20of%20Waves "0, 0, 0") ; Clear Value
  (bind _displacement (CallFunction|CreateWaveSet Location _wave_direction_v2 Time _global_wave_settings (Variables|Default|GetWave%20Set%2001))) ; Generate Wave Set 1
  (LocalVariables|SetSum%20of%20Waves _displacement)
  (if (Variables|Default|GetUse%20Wave%20Set%2002)
    (bind _displacement_2 (CallFunction|CreateWaveSet Location _wave_direction_v2 Time _global_wave_settings (Variables|Default|GetWave%20Set%2002))) ; Generate Wave Set 2
    (LocalVariables|SetSum%20of%20Waves (/ (+ (LocalVariables|GetSum%20of%20Waves) _displacement_2) 2.0)) ; Wave Set 1 + 2
  )
  (return (LocalVariables|GetSum%20of%20Waves)))

(fn ProcessBuoyancy
  (params (Component :type Primitive%20Component%20Object%20Reference) (Actor%20Transform :type Transform) (Point%20Location :type Vector) (Mass :type Float%20%28single-precision%29) (Thickness :type Float%20%28single-precision%29) (Displace%20Ratio :type Float%20%28single-precision%29) (Time :type Float%20%28single-precision%29))
  (bind _returnvalue (Math|Transform|TransformLocation Actor%20Transform Point%20Location))
  ;[1 1 1] Process Wave Height Data for Point Buoyancy
  (bind (_is_under_water _amount) (CallFunction|FindWaveHeightatPoint Actor%20Transform Point%20Location Thickness (* Time (Variables|Default|GetTime%20Multiplier))))
  (if _is_under_water
    (Class|PrimitiveComponent|AddForceatLocation Component (* (* (Math|Vector|MakeVector 0.0 0.0 (* (Variables|Default|GetWater%20Density) Displace%20Ratio)) Mass) _amount) _returnvalue "None") ; Apply Upwards (Buoyancy) Force
    (else
      (Class|PrimitiveComponent|AddForceatLocation Component (* (* (Math|Vector|MakeVector 0.0 0.0 -9.8e+02) Mass) _amount) _returnvalue "None") ; Apply Downwards (Gravity) Force
    ))
  (return _is_under_water))

(fn FindWaveHeightatPoint
  (params (Transform :type Transform) (Location :type Vector) (Thickness :type Float%20%28single-precision%29) (Time :type Float%20%28single-precision%29))
  (bind _returnvalue (Math|Transform|TransformLocation Transform Location))
  (bind _z (Math|Vector|BreakVector _returnvalue))
  ;[1 1 1] Find the Wave Height at a Given Location
  (bind _height_at_location (CallFunction|GetWaveHeight _returnvalue Time))
  (return (> (- (.Z (Math|Vector|BreakVector _height_at_location)) _z) 0.0) (Math|Float|Absolute(Float) (Math|Float|Clamp(Float) (Math|Float|Power (/ (- (.Z (Math|Vector|BreakVector _height_at_location)) _z) Thickness) 2.0))) (- (.Z (Math|Vector|BreakVector _height_at_location)) _z) (Math|Vector|MakeVector (.X (Math|Vector|BreakVector (+ _returnvalue _height_at_location))) (.Y (Math|Vector|BreakVector (+ _returnvalue _height_at_location))) _z) (.Z (Math|Vector|BreakVector _height_at_location))))

(fn InitGlobalParameters
  ;[1 1 1] Retrieve the Global Parameters
  (Utilities|FlowControl|Sequence
    (:then_0
      (bind _returnvalue (Rendering|Material|GetScalarParameterValue 0 "WaveSetRotation" :!class /Script/Engine.KismetMaterialLibrary))
      (LocalVariables|SetRotation _returnvalue))
    (:then_1
      (bind _returnvalue_2 (Rendering|Material|GetScalarParameterValue 0 "WaveSetLength" :!class /Script/Engine.KismetMaterialLibrary))
      (LocalVariables|SetLength _returnvalue_2))
    (:then_2
      (bind _returnvalue_3 (Rendering|Material|GetScalarParameterValue 0 "WaveSetAmplitude" :!class /Script/Engine.KismetMaterialLibrary))
      (LocalVariables|SetAmplitude _returnvalue_3))
    (:then_3
      (bind _returnvalue_4 (Rendering|Material|GetScalarParameterValue 0 "WaveSetSteepness" :!class /Script/Engine.KismetMaterialLibrary))
      (LocalVariables|SetSteepness _returnvalue_4))
    (:then_4
      (bind _returnvalue_5 (Rendering|Material|GetScalarParameterValue 0 "WaveSetTimeMultiplier" :!class /Script/Engine.KismetMaterialLibrary))
      (LocalVariables|SetTimeMultiplier _returnvalue_5))
    (:then_5
      (Variables|Default|SetGlobal%20Wave%20Settings (Utilities|Struct|MakeWaveParameters (LocalVariables|GetRotation) (LocalVariables|GetLength) (LocalVariables|GetAmplitude) (LocalVariables|GetSteepness) (LocalVariables|GetTimeMultiplier))))
    (:then_6
      (bind _returnvalue_6 (Rendering|Material|GetVectorParameterValue 0 "WavesDirectionV2" :!class /Script/Engine.KismetMaterialLibrary))
      (Variables|Default|SetWave%20Direction%20V2 (Math|Vector|MakeVector (.R (Math|Color|BreakColor _returnvalue_6)) (.G (Math|Color|BreakColor _returnvalue_6)) 0.0)))
    (:then_7
      (bind _returnvalue_7 (Rendering|Material|GetScalarParameterValue 0 "UseWaveSet02" :!class /Script/Engine.KismetMaterialLibrary))
      (Variables|Default|SetUse%20Wave%20Set%2002 (Math|Conversions|ToBoolean(Integer) (Math|Float|Floor _returnvalue_7))))))