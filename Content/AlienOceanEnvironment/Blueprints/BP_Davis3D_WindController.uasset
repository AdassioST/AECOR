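; BP_Davis3D_WindController is a wind controller that feeds the MPC_AlienOcean material parameter collection for the alien ocean environment.
; BeginPlay writes the wind speed and scale parameters.
; Three timelines are built to animate intensity, rotation and accumulated UV offsets, with rotation splitting the scroll between X and Y.
; No graph event starts these timelines, so they depend on autoplay or external triggering, neither shown here.
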(event EventBeginPlay
  (Rendering|Material|SetScalarParameterValue "/Game/AlienOceanEnvironment/Materials/MPC_AlienOcean.MPC_AlienOcean" "WindSpeed" (Variables|Default|GetWindSpeed) :!class /Script/Engine.KismetMaterialLibrary)
  (Rendering|Material|SetScalarParameterValue "/Game/AlienOceanEnvironment/Materials/MPC_AlienOcean.MPC_AlienOcean" "WindScale" (Variables|Default|GetWindScale) :!class /Script/Engine.KismetMaterialLibrary))

(fn ConstructionScript)