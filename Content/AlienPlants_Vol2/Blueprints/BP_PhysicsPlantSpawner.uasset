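; Spawner that swaps nearby instanced foliage for matching physics plant Blueprints during play.
; Each Tick sphere-traces around its parent component within PhysicsRadius, which BeginPlay also writes to the MPC_FoliagePhysics parameter collection.
; A macro matches hit instances to FoliageBlueprints by name, stripping "BP_" and "_C" from class names.
; A DoOnce gates spawning, and each instance is removed only once its replacement is valid, avoiding visual hitches.
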(event EventBeginPlay
  (Rendering|Material|SetScalarParameterValue "/Game/AlienPlants_Vol2/Materials/MaterialFunctions/MPC_FoliagePhysics.MPC_FoliagePhysics" "PhysicsRadius" (Variables|Default|GetPhysicsRadius) :!class /Script/Engine.KismetMaterialLibrary))

(event EventTick
  (params (DeltaSeconds :type Float%20%28single-precision%29))
  (bind _returnvalue (Class|Actor|GetParentComponent))
  (bind _returnvalue_2 (Transformation|GetWorldLocation _returnvalue))
  (CallFunction|ResetPlantSpawn)
  (bind (_outhits _returnvalue_3) (Collision|MultiSphereTraceByChannel _returnvalue_2 (- _returnvalue_2 "0, 0,1.000000") (Variables|Default|GetPhysicsRadius) "TraceTypeQuery1" false 0 "None"))
  (if _returnvalue_3
    (for _array_element _outhits
      (if (.bBlockingHit (Collision|BreakHitResult _array_element))
        (bind _asinstanced_static_mesh_component (Utilities|Casting|CastToInstancedStaticMeshComponent (.HitComponent (Collision|BreakHitResult _array_element)))) ; Did it hit a foliage actor?
        (|FindandReplaceFoliagewithBlueprint _asinstanced_static_mesh_component (.OutInstanceTransform (Components|InstancedStaticMesh|GetInstanceTransform _asinstanced_static_mesh_component (.HitItem (Collision|BreakHitResult _array_element)) false)) (.HitComponent (Collision|BreakHitResult _array_element)) (.HitItem (Collision|BreakHitResult _array_element)))))))

(fn ConstructionScript)

(event Custom|Reset_PlantSpawn
  (Utilities|FlowControl|DoOnce false) ; enters at Reset
)