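; Physics-interactive wheat plant actor that stands in for an instanced foliage mesh while the player is near.
; Overlap by the player or a "Physics"-tagged actor simulates the skeletal mesh's bones below the base.
; A delay loop compares player distance to the radius from MPC_FoliagePhysics.
; Once out of range, a timeline drives physics blend weight, then the actor adds a matching instance to the foliage actor and destroys itself.
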(event OnComponentBeginOverlap(Sphere)
  (params (OverlappedComponent :type Primitive%20Component%20Object%20Reference) (OtherActor :type Actor%20Object%20Reference) (OtherComp :type Primitive%20Component%20Object%20Reference) (OtherBodyIndex :type Integer) (bFromSweep :type Boolean) (SweepResult :type Hit%20Result%20Structure%20%28by%20ref%29))
  (if (or (== OtherActor (Game|Player|GetPlayerPawn 0)) (Actor|ActorHasTag OtherActor "Physics"))
    ;[1 1 1] Simulate Physics
    (Class|SkeletalMeshComponent|SetAllBodiesBelowSimulatePhysics (Variables|Default|GetSK_APV2_Wheat) (Utilities|String|StringToName "b_Base") true false)))

(event EventBeginPlay
  (bind _sk_apv2_wheat (Variables|Default|GetSK_APV2_Wheat))
  (bind _returnvalue (Rendering|Material|GetScalarParameterValue "/Game/AlienPlants_Vol2/Materials/MaterialFunctions/MPC_FoliagePhysics.MPC_FoliagePhysics" "PhysicsRadius" :!class /Script/Engine.KismetMaterialLibrary))
  (Variables|Default|SetPhysicsRadius _returnvalue)
  ;[1 1 1] Get reference to Foliage World Actor
  (bind _outactors (Actor|GetAllActorsOfClass "/Script/Foliage.InstancedFoliageActor"))
  (Variables|Default|SetWorldFoliage (Utilities|Array|Get(acopy) _outactors))
  (Utilities|FlowControl|Delay 0.1 :!label _label)
  (if (> (Transformation|GetDistanceTo (Game|GetPlayerCharacter 0) self) (+ (Variables|Default|GetPhysicsRadius) 1e+02))
    (Utilities|FlowControl|DoOnce false
      (:Completed
        (bind _newtrack_0 (Timeline|Timeline_0 PlayFromStart)
          (:Update
            (bind _output_get (Variables|Default|SetPhysicsAlpha _newtrack_0))
            (Class|SkeletalMeshComponent|SetAllBodiesBelowPhysicsBlendWeight (Variables|Default|GetSK_APV2_Wheat) (Utilities|String|StringToName "b_Stem1") _output_get false true))
          (:Finished
            (Collision|SetCollisionEnabled _sk_apv2_wheat "NoCollision")
            (Physics|SetSimulatePhysics _sk_apv2_wheat false)
            (for (_array_element _array_index) (Actor|GetComponentsByClass (Variables|Default|GetWorldFoliage) "/Script/Engine.InstancedStaticMeshComponent")
              (if (Utilities|String|Contains (Utilities|GetDisplayName _array_element) "APV2_Wheat")
                (Variables|Default|SetClassIndex _array_index)))
            (Utilities|FlowControl|DoOnce false
              (:Completed
                (Components|InstancedStaticMesh|AddInstance (Utilities|Array|Get(acopy) (Actor|GetComponentsByClass (Variables|Default|GetWorldFoliage) "/Script/Engine.InstancedStaticMeshComponent") (Variables|Default|GetClassIndex)) (Transformation|GetWorldTransform (Variables|Default|GetSK_APV2_Wheat)))
                (Actor|DestroyActor)))))))
    (else
      (goto _label))))

(fn ConstructionScript)