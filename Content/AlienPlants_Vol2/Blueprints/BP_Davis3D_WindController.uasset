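; Wind controller Blueprint for the alien plants pack, writing wind settings to the MPC_APV2 material parameter collection.
; BeginPlay pushes wind speed and scale.
; Three timelines handle animated wind: one sets rotation, which splits another's accumulated UV offset between X and Y, and one modulates intensity.
; No graph wire starts these timelines, so their updates depend on autoplay, which the graph does not show.
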(event EventBeginPlay
  (Rendering|Material|SetScalarParameterValue "/Game/AlienPlants_Vol2/Materials/MaterialFunctions/MPC_APV2.MPC_APV2" "WindSpeed" (Variables|Default|GetWindSpeed) :!class /Script/Engine.KismetMaterialLibrary)
  (Rendering|Material|SetScalarParameterValue "/Game/AlienPlants_Vol2/Materials/MaterialFunctions/MPC_APV2.MPC_APV2" "WindScale" (Variables|Default|GetWindScale) :!class /Script/Engine.KismetMaterialLibrary))

(fn ConstructionScript)